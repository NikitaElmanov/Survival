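; BP_BoxModel_Forgame is an interactable box prefab that inherits its behavior from a parent Blueprint.
; Its Interact override casts the character to SurvivalCharacterPlayer, then passes it through an always-true branch to the parent Interact and returns that success flag and message.
; A disconnected check of the player's pickaxe pickup, weapon pickup and weapon repair objectives remains in the graph but does not gate interaction.
; The event graph and construction script add no logic.
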(fn `Interact`
  (params (Character :type "/Game/Blueprints/Characters/SurvivalCharacter Object Reference"))
  (returns (Successfull :type Boolean) (Message :type String))
  (locals (L_Character :type "/Game/Blueprints/Characters/SurvivalCharacterPlayer Object Reference"))
  (bind _assurvival_character_player (cast `/Game/Blueprints/Characters/SurvivalCharacterPlayer` Character))
  (bind _output_get (set `local.L_Character` _assurvival_character_player))
  (if true
    (bind (_successfull _message) (`parent.Interact` (`local.L_Character`)))
    (return _successfull _message)))

(fn `UserConstructionScript`
  (`parent.UserConstructionScript`))