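; BP_Rock is a mineable rock prefab that yields rock items when struck with a pickaxe.
; Point damage calls RockHit, which ignores any damage causer that is not exactly a BP_Pickaxe.
; Each valid hit decrements a hit counter and spawns a BP_ItemRock at the hit location with a random uniform scale.
; The rock destroys itself once the counter runs out.
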(event `self.ReceivePointDamage`
  (params (Damage :type "Float (single-precision)") (DamageType :type "DamageType Object Reference") (HitLocation :type "Vector Structure") (HitNormal :type "Vector Structure") (HitComponent :type "PrimitiveComponent Object Reference") (BoneName :type Name) (ShotFromDirection :type "Vector Structure") (InstigatedBy :type "Controller Object Reference") (DamageCauser :type "Actor Object Reference") (HitInfo :type "HitResult Structure (by ref)"))
  (`self.RockHit` HitLocation DamageCauser))

(fn `RockHit`
  (params (HitLocation :type "Vector Structure") (DamageCauser :type "Object Object Reference"))
  (locals (L_ItemRock :type "/Game/Blueprints/Storage/Items/BP_ItemRock Object Reference") (L_CurrentRandomRockScaleToSpawn :type "Float (double-precision)" :default 0.0) (L_HitLocation :type "Vector Structure"))
  (set `local.L_HitLocation` HitLocation)
  (if (== (`GameplayStatics.GetObjectClass` DamageCauser) "/Game/Blueprints/Storage/Items/Equipables/Weapons/BP_Pickaxe.BP_Pickaxe_C")
    (`/Engine/EditorBlueprintResources/StandardMacros.DecrementInt` (`self.RockIntegers`)
      (:`  `
        (bind _output_get (set `local.L_CurrentRandomRockScaleToSpawn` (`KismetMathLibrary.RandomFloatInRange` (`self.MinRockScaleToSpawn`) (`self.MaxRockScaleToSpawn`))))
        (bind _returnvalue (`|SpawnActorFromClass` "/Game/Blueprints/Storage/Items/BP_ItemRock.BP_ItemRock_C" (`KismetMathLibrary.MakeTransform` (`local.L_HitLocation`) (struct) (`KismetMathLibrary.MakeVector` _output_get _output_get _output_get)) "AdjustIfPossibleButAlwaysSpawn" "OverrideRootScale" null 1 null))
        (set `local.L_ItemRock` _returnvalue)
        (if (<= (`self.RockIntegers`) 0)
          (`self.K2_DestroyActor`))))))

(fn `UserConstructionScript`)