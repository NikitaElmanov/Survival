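; Double-door prefab that the survival player opens by interacting with either door mesh, and that closes when an overlap with its trigger ends.
; Interact checks the player's hit component, then fires a dispatcher, bound on BeginPlay, that plays the rotation timeline.
; The sign of the player's world-space forward X sets the swing direction, with the two door roots mirrored.
; Ending the overlap reverses the timeline, clearing Opened when finished.
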(event `self.ReceiveBeginPlay`
  (add `self.OnAllowToOpneDoors` (delegate `OnAllowToOpneDoors_OpenEvent`)))

(event `OnAllowToOpneDoors_OpenEvent` :!signature `self.OnAllowToOpneDoors`
  (params (`Co-DirectionalWithX` :type Boolean))
  (bind _currentrotationz (`self.CurrentRotationZ`))
  (set `self.Co-DirectionWithX` `Co-DirectionalWithX`)
  (bind (_direction _rotationz) (`Timeline|RotationDoors` :!label _label)
    (:`Update`
      (bind _output_get (set `self.CurrentRotationZ` _rotationz))
      (`SceneComponent.K2_SetRelativeRotation` (`self.SceneRootDoor_1`) (`KismetMathLibrary.MakeRotator` 0.0 0.0 (select `bool` (`self.Co-DirectionWithX`) :`false` _output_get :`true` (* -1 _output_get))) false false)
      (`SceneComponent.K2_SetRelativeRotation` (`self.SceneRootDoor_2`) (`KismetMathLibrary.MakeRotator` 0.0 0.0 (select `bool` (`self.Co-DirectionWithX`) :`false` (* -1 _currentrotationz) :`true` _currentrotationz)) false false))
    (:`Finished`
      ;[1 1 1] Toggle status of doors animation
      (bind _output_get_2 (set `self.TimelineDirection` _direction))
      (if (`|EnumEquality` _output_get_2 "Backward")
        (set `self.Opened` false)))))

(event `self.TriggerToCloseDoors.OnComponentEndOverlap`
  (params (OverlappedComponent :type "PrimitiveComponent Object Reference") (OtherActor :type "Actor Object Reference") (OtherComp :type "PrimitiveComponent Object Reference") (OtherBodyIndex :type Integer))
  (if (`self.Opened`)
    (goto _label :!via `Reverse`)))

(fn `Interact`
  (params (Character :type "/Game/Blueprints/Characters/SurvivalCharacter Object Reference"))
  (returns (Successfull :type Boolean) (Message :type String))
  (bind _assurvival_character_player (cast `/Game/Blueprints/Characters/SurvivalCharacterPlayer` Character)
    (:`then`
      (bind _output_get (set `self.Character` _assurvival_character_player))
      (bind (_bblockinghit _binitialoverlap _time _distance _location _impactpoint _normal _impactnormal _physmat _hitactor _hitcomponent) (`GameplayStatics.BreakHitResult` (`/Game/Blueprints/Characters/SurvivalCharacter.GetInteractionInfo` _output_get (`/Game/Blueprints/Characters/SurvivalCharacterPlayer.DistanceToEquip` _output_get))))
      (if (or (== (`self.Door_1`) _hitcomponent) (== _hitcomponent (`self.Door_2`)))
        (`self.OnAllowToOpneDoors` (> (.x (`self.GetActorForwardVector` (`self.Character`))) 0.0))
        (set `self.Opened` true)
        (return true "")
        (else
          (return false "Interact only doors"))))
    (:`CastFailed`
      (return false "Character is not Survival Character Player"))))

(fn `UserConstructionScript`)