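; Choppable tree that yields wood, with wood count and scale randomized at construction.
; Axe damage lowers its condition until it falls and a timeline rolls it over, while other damage spawns berries nearby.
; Any hit also enables physics on the tree mesh.
; Interacting with a fallen tree adds wood to the character's storage and destroys it, and an interaction widget hints that an axe is needed.
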(event `self.ReceiveAnyDamage`
  (params (Damage :type "Float (single-precision)") (DamageType :type "DamageType Object Reference") (InstigatedBy :type "Controller Object Reference") (DamageCauser :type "Actor Object Reference"))
  (`self.Hit a tree` Damage InstigatedBy DamageCauser)
  (`PrimitiveComponent.SetSimulatePhysics` (`self.tree`) true))

(event `self.ReceiveBeginPlay`
  ;[1 1 1] Tree falling animation
  (add `self.onTreeFell` (delegate `PlayFallAnim`)))

(event `PlayFallAnim` :!signature `self.onTreeFell`
  (params (Tree :type "/Game/Blueprints/Prefabs/BP_Tree Object Reference") (Instigator :type "Pawn Object Reference"))
  (bind _returnvalue_roll (`KismetMathLibrary.BreakRotator` (`self.K2_GetActorRotation`)))
  (bind (_returnvalue_roll_2 _returnvalue_pitch _returnvalue_yaw) (`KismetMathLibrary.BreakRotator` (`self.K2_GetActorRotation`)))
  (bind (_returnvalue_roll_3 _returnvalue_pitch_2 _returnvalue_yaw_2) (`KismetMathLibrary.BreakRotator` (`self.K2_GetActorRotation`)))
  ;[1 1 1] Tree falling animation
  (bind _assurvival_character_player (cast `/Game/Blueprints/Characters/SurvivalCharacterPlayer` Instigator))
  (bind _output_get (set `self.SurvavialCaharacter` _assurvival_character_player))
  (set `self.SurvivalCharacterDirection` (`self.GetActorForwardVector` _output_get))
  (bind (_direction _newtrack_0) (`Timeline|Timeline_0`)
    (:`Update`
      (bind _returnvalue (+ _returnvalue_roll _newtrack_0))
      (if (`KismetMathLibrary.InRange_FloatFloat` _returnvalue -90.0 90.0)
        (`self.K2_SetActorRotation` (`KismetMathLibrary.MakeRotator` _returnvalue _returnvalue_pitch_2 _returnvalue_yaw_2))
        (`self.K2_SetActorRotation` (`KismetMathLibrary.MakeRotator` _returnvalue_roll_2 _returnvalue_pitch _returnvalue_yaw))))))

(fn `Hit a tree`
  (params (InputPin :type "Float (double-precision)") (Instigator :type "Controller Object Reference") (Causer :type "Object Object Reference"))
  (returns (Fallen :type Boolean) (Damaged :type Boolean))
  (bind _sphere (`self.Sphere`))
  (bind _returnvalue (* (* (`KismetMathLibrary.RandomUnitVector`) (1.0 1.0 0.0)) (`KismetMathLibrary.RandomFloatInRange` 5.0 (* (`SphereComponent.SphereRadius` _sphere) (`SphereComponent.GetShapeScale` _sphere)))))
  (if (== (`GameplayStatics.GetObjectClass` Causer) "/Game/Blueprints/Storage/Items/Equipables/Weapons/BP_AxeModel.BP_AxeModel_C")
    (bind _output_get (set `self.Condition` (- (`self.Condition`) InputPin)))
    (if (<= _output_get 0.0)
      (set `self.Fallen` true)
      (`self.onTreeFell` self (`Controller.K2_GetPawn` Instigator))
      (return true true)
      (else
        (return false true)))
    (else
      ;[1 1 1] DROP BERRIES [attach to Branch(false)]
      (`KismetSystemLibrary.PrintString` (`KismetStringLibrary.Conv_VectorToString` _returnvalue))
      (`|SpawnActorFromClass` "/Game/Blueprints/Storage/Items/Food/Food_Berries.Food_Berries_C" (`KismetMathLibrary.MakeTransform` (+ _returnvalue (`SceneComponent.K2_GetComponentLocation` (`self.Sphere`))) (struct) (0.05 0.05 0.05)) "AlwaysSpawn" "OverrideRootScale" null 1 null)
      (return false false))))

(fn `Interact`
  (params (Character :type "/Game/Blueprints/Characters/SurvivalCharacter Object Reference"))
  (returns (Successfull :type Boolean) (Message :type String))
  (if (`self.Fallen`)
    (`/Game/Blueprints/Storage/BP_StorageComponent.CreateItems` (`/Game/Blueprints/Characters/SurvivalCharacter.BP_StorageComponent` Character) (`|MakeArray` (make `/Game/Blueprints/Storage/ST_BeginItemInfo` "/Game/Blueprints/Storage/Items/BP_Wood.BP_Wood_C" (`self.WoodCount`))))
    (`self.K2_DestroyActor`)
    (`/Engine/EditorBlueprintResources/StandardMacros.IsValid` (`self.InteractWidget`)
      (:`Is Valid`
        (`Widget.RemoveFromParent` (`self.InteractWidget`))
        (return true "")))
    (else
      (return false "Tree is not fallen"))))

(fn `ToggleInteractAttampt`
  (params (Enable :type Boolean))
  (returns (ReturnValue :type Boolean))
  (if Enable
    (bind _returnvalue (`|CreateWidget` "/Game/UI/InteractionWidgets/W_InteractionInfo-SimpleMessage.W_InteractionInfo-SimpleMessage_C" null "Use \"Axe\" to get a wood"))
    (bind _output_get (set `self.InteractWidget` _returnvalue))
    (`UserWidget.AddToViewport` _output_get 0)
    (return false)
    (else
      (`/Engine/EditorBlueprintResources/StandardMacros.IsValid` (`self.InteractWidget`)
        (:`Is Valid`
          (`Widget.RemoveFromParent` (`self.InteractWidget`))
          (set `self.InteractWidget` null)
          (return false))))))

(fn `UserConstructionScript`
  (set `self.WoodCount` (`KismetMathLibrary.RandomIntegerInRange` (`self.MinWoodCount`) (`self.MaxWoodCount`)))
  (`SceneComponent.SetRelativeScale3D` (`self.tree`) (* (1.0 1.0 1.0) (`KismetMathLibrary.RandomFloatInRange` 0.4 1.0))))