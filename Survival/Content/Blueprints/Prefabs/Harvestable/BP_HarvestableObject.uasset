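; Base harvestable world object that gives its configured items to an interacting character's storage once.
; Interact calls Harvest with the character's storage component if not yet harvested, otherwise fails with an "Already harvested" message.
; Harvest creates the items in storage, resets the item list to its first item at zero count, fires OnItemsHarvested and sets the Harvested flag.
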(fn `Harvest`
  (params (StorageComponent :type "/Game/Blueprints/Storage/BP_StorageComponent Object Reference"))
  (bind _output_item (break `/Game/Blueprints/Storage/ST_BeginItemInfo` (`|GetArrayItem` (`self.ItemsToHarvest`))))
  (bind _createditems (`/Game/Blueprints/Storage/BP_StorageComponent.CreateItems` StorageComponent (`self.ItemsToHarvest`)))
  (set `self.ItemsToHarvest` (`|MakeArray` (make `/Game/Blueprints/Storage/ST_BeginItemInfo` _output_item)))
  (`self.OnItemsHarvested` StorageComponent _createditems)
  (set `self.Harvested` true))

(fn `Interact`
  (params (Character :type "/Game/Blueprints/Characters/SurvivalCharacter Object Reference"))
  (returns (Successfull :type Boolean) (Message :type String))
  (if (not (`self.Harvested`))
    (`self.Harvest` (`/Game/Blueprints/Characters/SurvivalCharacter.BP_StorageComponent` Character))
    (return true "")
    (else
      (return false "Already harvested"))))

(fn `UserConstructionScript`)