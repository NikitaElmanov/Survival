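; Harvestable berry bush that regrows its berries after items are harvested from it.
; On BeginPlay it binds to the items-harvested event, which starts a looping timer on RecoverBerries using the berry recovery time.
; Each tick of that timer clears the Harvested flag and rebuilds the first harvest entry with one more berry until the bush maximum is reached.
; The timer is never cleared here, even at the maximum.
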(event `self.ReceiveBeginPlay`
  (`parent.ReceiveBeginPlay`)
  (add `self.OnItemsHarvested` (delegate `OnItemsHarvested_Event`)))

(event `OnItemsHarvested_Event` :!signature `self.OnItemsHarvested`
  (params (StorageComponent :type "/Game/Blueprints/Storage/BP_StorageComponent Object Reference") (Items :type "Array of /Game/Blueprints/Storage/Items/BP_StorageItem Object Reference (by ref)"))
  (`KismetSystemLibrary.K2_SetTimer` null "RecoverBerries" (`self.BerriesRecoverTime`) true))

(fn `RecoverBerries`
  (bind (_output_item _output_count) (break `/Game/Blueprints/Storage/ST_BeginItemInfo` (`|GetArrayItem` (`self.ItemsToHarvest`))))
  (bind (_output_item_2 _output_count_2) (break `/Game/Blueprints/Storage/ST_BeginItemInfo` (`|GetArrayItem` (`self.ItemsToHarvest`))))
  (set `self.Harvested` false)
  (if (< _output_count (`self.MaxBerriesOnBush`))
    (set `self.ItemsToHarvest` (`|MakeArray` (make `/Game/Blueprints/Storage/ST_BeginItemInfo` _output_item_2 (+ _output_count_2 1))))))

(fn `UserConstructionScript`
  (`parent.UserConstructionScript`))