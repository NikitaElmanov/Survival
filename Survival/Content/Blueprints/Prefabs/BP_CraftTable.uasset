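; Interactable crafting table for the survival game that opens a crafting interface for the player.
; Interact casts the character's controller to SurvivalPlayerController, requests its craft widget and initializes it with the table's storage and craft components, failing with a message for other controllers.
; ToggleInteractAttampt creates or removes the "Press E to craft" prompt, which Interact also clears after a validity check.
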(fn `Interact`
  (params (Character :type "/Game/Blueprints/Characters/SurvivalCharacter Object Reference"))
  (returns (Successfull :type Boolean) (Message :type String))
  (bind _assurvival_player_controller (cast `/Game/Blueprints/GameMode/SurvivalPlayerController` (`Pawn.GetController` Character))
    (:`then`
      (bind _craftwidget (`/Game/Blueprints/GameMode/SurvivalPlayerController.CraftWidget` _assurvival_player_controller true))
      (`/Game/UI/Craft/WB_CraftWindow.InitCraftInterface` _craftwidget (`self.BP_StorageComponent`) (`self.BP_CraftComponent`))
      (`/Engine/EditorBlueprintResources/StandardMacros.IsValid` null
        (:`Is Valid`
          (`Widget.RemoveFromParent` (`self.InteractionWidget`))
          (return true ""))))
    (:`CastFailed`
      (return false "Character is not controlled by player"))))

(fn `ToggleInteractAttampt`
  (params (Enable :type Boolean))
  (returns (ReturnValue :type Boolean))
  (locals (InteractWidget :type "/Game/UI/InteractionWidgets/W_InteractionInfo-SimpleMessage Object Reference"))
  (if Enable
    (bind _returnvalue (`|CreateWidget` "/Game/UI/InteractionWidgets/W_InteractionInfo-SimpleMessage.W_InteractionInfo-SimpleMessage_C" null "Press \"E\" to craft"))
    (bind _output_get (set `self.InteractionWidget` _returnvalue))
    (`UserWidget.AddToViewport` _output_get 0)
    (return true)
    (else
      (`/Engine/EditorBlueprintResources/StandardMacros.IsValid` (`self.InteractionWidget`)
        (:`Is Valid`
          (`Widget.RemoveFromParent` (`self.InteractionWidget`))
          (set `self.InteractionWidget` null)
          (return false))))))

(fn `UserConstructionScript`)