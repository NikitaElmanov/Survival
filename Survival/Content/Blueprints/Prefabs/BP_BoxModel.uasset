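; BP_BoxModel is an interactable storage box with an animated lid and an "E to open" prompt.
; Interact succeeds only while closed: it fires OnBoxOpened, clears Closed, registers the box with SurvivalPlayerController and passes its storage component to ExchangeWidget.
; A timeline rotates the cover open and reverses when the controller's OnBoxClosed names this box; Closed is not reset here.
; ToggleInteractAttampt creates or removes the prompt widget.
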(event `self.ReceiveBeginPlay`
  (add `self.OnBoxOpened` (delegate `BoxOpened`))
  (bind _assurvival_player_controller (cast `/Game/Blueprints/GameMode/SurvivalPlayerController` (`GameplayStatics.GetPlayerController` 0)))
  (add `/Game/Blueprints/GameMode/SurvivalPlayerController.OnBoxClosed` _assurvival_player_controller (delegate `BoxClosed`)))

(event `BoxOpened`
  (bind (_direction _rotation) (`Timeline|CoverRotation_open` :!label _label)
    (:`Update`
      (`SceneComponent.K2_SetRelativeRotation` (`self.CoverScene`) (`KismetMathLibrary.MakeRotator` _rotation) false false))))

(event `BoxClosed`
  (params (Box :type "/Game/Blueprints/Prefabs/BP_BoxModel Object Reference"))
  (if (== Box self)
    (goto _label :!via `Reverse`)))

(fn `Interact`
  (params (Character :type "/Game/Blueprints/Characters/SurvivalCharacter Object Reference"))
  (returns (Successfull :type Boolean) (Message :type String))
  (locals (L_SurvivalController :type "/Game/Blueprints/GameMode/SurvivalPlayerController Object Reference"))
  (bind _assurvival_player_controller (cast `/Game/Blueprints/GameMode/SurvivalPlayerController` (`Pawn.GetController` Character))
    (:`then`
      (set `local.L_SurvivalController` _assurvival_player_controller)
      ;[1 1 1] Play Cover opening animation
      (if (`self.Closed`)
        (`self.OnBoxOpened`)
        (set `self.Closed` false)
        (set `/Game/Blueprints/GameMode/SurvivalPlayerController.CurrentInteractedBox` self (`local.L_SurvivalController`))
        (`/Game/Blueprints/GameMode/SurvivalPlayerController.ExchangeWidget` (`local.L_SurvivalController`) (`self.BP_StorageComponent`) false)
        (return true "")
        (else
          _)))
    (:`CastFailed`
      _))
  (return false ""))

(fn `ToggleInteractAttampt`
  (params (Enable :type Boolean))
  (returns (ReturnValue :type Boolean))
  (if Enable
    (bind _returnvalue (`|CreateWidget` "/Game/UI/InteractionWidgets/W_InteractionInfo-SimpleMessage.W_InteractionInfo-SimpleMessage_C" null "Press \"E\" to open"))
    (bind _output_get (set `self.InteractWidget` _returnvalue))
    (`UserWidget.AddToViewport` _output_get 0)
    (return true)
    (else
      (`/Engine/EditorBlueprintResources/StandardMacros.IsValid` (`self.InteractWidget`)
        (:`Is Valid`
          (`Widget.RemoveFromParent` (`self.InteractWidget`))
          (set `self.InteractWidget` null)
          (return false))))))

(fn `UserConstructionScript`)