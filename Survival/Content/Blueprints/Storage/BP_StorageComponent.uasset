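; Inventory component that gives its owner a paged grid storage with a weight limit, seeded on BeginPlay with fixed and chance-rolled items.
; Items are spawned actors; adding checks weight and scans for free multi-cell slots, then merges stackables into the first same-class item.
; It also handles relocation, partial or full removal, transfers between storages and drops in front of the owner, signalling inventory updates and tracking total weight.
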(event `self.ReceiveBeginPlay`
  (`self.CreateItems` (`self.BeginItems`))
  (`self.CreateItems` (`self.GenerateRandomItems`))
  (add `Actor.OnDestroyed` (`self.GetOwner`) (`|CreateDelegate` :!event `DoOnOwnerDestroyed`)))

(fn `Add Item`
  (params (Item :type "/Game/Blueprints/Storage/Items/BP_StorageItem Object Reference"))
  (returns (Added :type Boolean))
  (locals (L_Item :type "/Game/Blueprints/Storage/Items/BP_StorageItem Object Reference") (L_X :type Integer :default 0) (L_Y :type Integer :default 0) (L_Page :type Integer :default 1))
  (bind _l_item (`local.L_Item`))
  (bind (_stackin _canbestacked) (`self.CheckItemsForStack` (`local.L_Item`)))
  (bind _output_get (set `local.L_Item` Item))
  (bind (_canbeadded _x _y _page) (`self.CheckIfItemCanBeAdded` _output_get))
  (if _canbeadded
    (set `local.L_X` _x)
    (set `local.L_Y` _y)
    (set `local.L_Page` _page)
    (if _canbestacked
      (`self.StackItem` (`local.L_Item`) _stackin)
      (`/Game/Blueprints/Storage/Items/BP_StorageItem.DestroyItem` (`local.l_item`))
      (`self.InventoryUpdated`)
      (return true)
      (else
        ;[1 1 1] Add New Item
        (`KismetArrayLibrary.Array_Add` (`self.Items`) _l_item)
        (`self.ChangeTotalWeight` (`/Game/Blueprints/Storage/Items/BP_StorageItem.GetTotalWeight` _l_item true 0))
        (`/Game/Blueprints/Storage/Items/BP_StorageItem.Item Added to Storage` (`local.L_Item`) self (`local.L_X`) (`local.L_Y`) (`local.L_Page`))
        (`self.InventoryUpdated`)
        (return true)))
    (else
      (return false))))

(fn `ChangeItemLocation`
  (params (Item :type "/Game/Blueprints/Storage/Items/BP_StorageItem Object Reference") (X :type Integer) (Y :type Integer) (Page :type Integer))
  (returns (Changed :type Boolean))
  (locals (L_Item :type "/Game/Blueprints/Storage/Items/BP_StorageItem Object Reference") (L_X :type Integer) (L_Y :type Integer) (L_Page :type Integer))
  (bind _output_get (set `local.L_Item` Item))
  (bind _output_get_2 (set `local.L_X` X))
  (bind _output_get_3 (set `local.L_Y` Y))
  (bind _output_get_4 (set `local.L_Page` Page))
  (bind _slotsarefree (`self.Check Slots For Item` _output_get _output_get_2 _output_get_3 _output_get_4))
  (if _slotsarefree
    (`/Game/Blueprints/Storage/Items/BP_StorageItem.RelocateItem` (`local.L_Item`) (`local.L_X`) (`local.L_Y`) (`local.L_Page`))
    (`self.InventoryUpdated`)
    (return true)
    (else
      (return false))))

(fn `ChangeTotalWeight`
  (params (Value :type "Float (double-precision)"))
  (set `self.StorageTotalWeight` (+ Value (`self.StorageTotalWeight`))))

(fn `Check Slots For Item`
  (params (Item :type "/Game/Blueprints/Storage/Items/BP_StorageItem Object Reference") (X :type Integer) (Y :type Integer) (Page :type Integer) (`Ignore Self` :type Boolean))
  (returns (SlotsAreFree :type Boolean))
  (locals (L_Item :type "/Game/Blueprints/Storage/Items/BP_StorageItem Object Reference") (L_X :type Integer) (L_Page :type Integer) (L_Y :type Integer) (CurIndexY :type Integer) (CurIndexX :type Integer) (L_IgnoreSelf :type Boolean))
  (bind (_page _x _y _sizex _sizey) (`/Game/Blueprints/Storage/Items/BP_StorageItem.Get Location in Inventory` (`local.L_Item`)))
  (bind _output_get (set `local.L_Item` Item))
  (`/Engine/EditorBlueprintResources/StandardMacros.IsValid` _output_get
    (:`Is Valid`
      (set `local.L_X` X)
      (set `local.L_Y` Y)
      (set `local.L_Page` Page)
      (set `local.L_IgnoreSelf` `Ignore Self`)
      (for _index (range _sizey)
        (set `local.CurIndexY` _index)
        (for _index_2 (range _sizex)
          (set `local.CurIndexX` _index_2)
          (bind (_item _free) (`self.CheckSlot` (`local.L_Page`) (+ (`local.CurIndexX`) (`local.L_X`)) (+ (`local.CurIndexY`) (`local.L_Y`))))
          (if (and (not _free) (!= _item (`local.L_Item`)))
            (return false))))
      (return true))
    (:`Is Not Valid`
      (return false))))

(fn `CheckFreeSlotForItem`
  (params (Item :type "/Game/Blueprints/Storage/Items/BP_StorageItem Object Reference"))
  (returns (SlotAreFree :type Boolean) (X :type Integer) (Y :type Integer) (Page :type Integer))
  (locals (L_Item :type "/Game/Blueprints/Storage/Items/BP_StorageItem Object Reference") (L_Page :type Integer) (L_Y :type Integer) (L_X :type Integer) (L_SlotNoFreeBreak :type Boolean) (CurIndexY :type Integer) (CurIndexX :type Integer))
  (set `local.L_Item` Item)
  (for _index (range 1 (+ (`self.StorageSizePages`) 1))
    (set `local.L_Page` _index)
    (for _index_2 (range (`self.StorageSizeY`))
      (set `local.L_Y` _index_2)
      (for _index_3 (range (`self.StorageSizeX`))
        (set `local.L_X` _index_3)
        (bind (_item _free) (`self.CheckSlot` (`local.L_Page`) (`local.L_X`) (`local.L_Y`)))
        (if _free
          (bind _slotsarefree (`self.Check Slots For Item` (`local.L_Item`) (`local.L_X`) (`local.L_Y`) (`local.L_Page`)))
          (if _slotsarefree
            (return true (`local.L_X`) (`local.L_Y`) (`local.L_Page`)))))))
  (return false 0 0 0))

(fn `CheckIfItemCanBeAdded`
  (params (Item :type "/Game/Blueprints/Storage/Items/BP_StorageItem Object Reference"))
  (returns (CanBeAdded :type Boolean) (X :type Integer) (Y :type Integer) (Page :type Integer))
  (locals (L_Item :type "/Game/Blueprints/Storage/Items/BP_StorageItem Object Reference") (L_X :type Integer :default 0) (L_Y :type Integer :default 0) (L_Page :type Integer :default 0))
  (bind _output_get (set `local.L_Item` Item))
  (if (`self.CheckIfItemCanBeAddedByWeight` _output_get true)
    (bind (_slotarefree _x _y _page) (`self.CheckFreeSlotForItem` (`local.L_Item`)))
    (if _slotarefree
      (return true _x _y _page)
      (else
        _)))
  (return false 0 0 0))

(fn `CheckIfItemCanBeAddedByWeight`
  (params (Item :type "/Game/Blueprints/Storage/Items/BP_StorageItem Object Reference") (Total :type Boolean) (Count :type Integer))
  (returns (ReturnValue :type Boolean))
  (return (<= (+ (`self.StorageTotalWeight`) (`/Game/Blueprints/Storage/Items/BP_StorageItem.GetTotalWeight` Item Total Count)) (`self.StorageMaxWeight`))))

(fn `CheckItemsForStack`
  (params (Item :type "/Game/Blueprints/Storage/Items/BP_StorageItem Object Reference"))
  (returns (StackIn :type "/Game/Blueprints/Storage/Items/BP_StorageItem Object Reference") (CanBeStacked :type Boolean))
  (locals (L_Item :type "/Game/Blueprints/Storage/Items/BP_StorageItem Object Reference"))
  (bind (_item _wasfound) (`self.Get Item in Storage by Class` (`GameplayStatics.GetObjectClass` (`local.L_Item`))))
  (bind _output_get (set `local.L_Item` Item))
  (if (`/Game/Blueprints/Storage/Items/BP_StorageItem.CanBeStacked` _output_get)
    (return _item _wasfound)
    (else
      (return null false))))

(fn `CheckSlot`
  (params (Page :type Integer) (X :type Integer) (Y :type Integer) (CheckExactSlot :type Boolean))
  (returns (Item :type "/Game/Blueprints/Storage/Items/BP_StorageItem Object Reference") (Free :type Boolean))
  (locals (L_Page :type Integer) (L_X :type Integer) (L_Y :type Integer) (L_Item :type "/Game/Blueprints/Storage/Items/BP_StorageItem Object Reference") (L_CheckExactSlot :type Boolean))
  (bind _l_y (`local.L_Y`))
  (bind _l_x (`local.L_X`))
  (bind _l_item (`local.L_Item`))
  (bind _l_page (`local.L_Page`))
  (set `local.L_Page` Page)
  (set `local.L_X` X)
  (set `local.L_Y` Y)
  (set `local.L_CheckExactSlot` CheckExactSlot)
  (`|ExecutionSequence`
    (:`then_0`
      ;[1 1 1] Check for grid inventory borders
      (`|ExecutionSequence`
        (:`then_0`
          (if (or (> _l_page (`self.StorageSizePages`)) (< _l_page 1))
            (return null false)))
        (:`then_1`
          (if (or (>= _l_x (`self.StorageSizeX`)) (< _l_x 0))
            (return null false)))
        (:`then_2`
          (if (or (>= _l_y (`self.StorageSizeY`)) (< _l_y 0))
            (return null false)))))
    (:`then_1`
      (for _array_element (`self.Items`)
        (bind (_page _x _y) (`/Game/Blueprints/Storage/Items/BP_StorageItem.Get Location in Inventory` _array_element))
        (if (select `bool` (`local.L_CheckExactSlot`) :`false` (`/Game/Blueprints/Storage/Items/BP_StorageItem.CheckIfItemIsInSlot` _array_element (`local.L_X`) (`local.L_Y`) (`local.L_Page`)) :`true` (and (== _page (`local.L_Page`)) (== _x (`local.L_X`)) (== _y (`local.L_Y`))))
          (set `local.L_Item` _array_element)
          (break))))
    (:`then_2`
      (return _l_item (not (`KismetSystemLibrary.IsValid` _l_item))))))

(fn `CreateItems`
  (params (Items :type "Array of /Game/Blueprints/Storage/ST_BeginItemInfo Structure"))
  (returns (CreatedItems :type "Array of /Game/Blueprints/Storage/Items/BP_StorageItem Object Reference"))
  (locals (L_CreatedItems :type "Array of /Game/Blueprints/Storage/Items/BP_StorageItem Object Reference") (L_ItemInfo :type "/Game/Blueprints/Storage/ST_BeginItemInfo Structure"))
  (bind (_item _count) (break `/Game/Blueprints/Storage/ST_BeginItemInfo` (`local.L_ItemInfo`)))
  (for _array_element Items
    (set `local.L_ItemInfo` _array_element)
    (if (defaults `Object` (`.Item_13_A53D5A4948F713A82DCFFC95F9D7867E` (break `/Game/Blueprints/Storage/ST_BeginItemInfo` _array_element)))
      (bind _returnvalue (`|SpawnActorFromClass` _item (`KismetMathLibrary.MakeTransform` (0.0 0.0 0.0)) "AlwaysSpawn" "OverrideRootScale" null (`KismetMathLibrary.SelectInt` _count 1 (defaults `Object` _item)) null :!label _label))
      (`KismetArrayLibrary.Array_Add` (`local.L_CreatedItems`) _returnvalue)
      (bind _added (`self.Add Item` _returnvalue))
      (if (not _added)
        (`KismetArrayLibrary.Array_RemoveItem` (`local.L_CreatedItems`) _returnvalue)
        (`/Game/Blueprints/Storage/Items/BP_StorageItem.DestroyItem` _returnvalue))
      (else
        (for _ (range 1 (+ (`.Count_15_F511CDE2445D8A55751FED878F1B0896` (break `/Game/Blueprints/Storage/ST_BeginItemInfo` (`local.L_ItemInfo`))) 1))
          (goto _label)))))
  (return (`local.L_CreatedItems`)))

(fn `DoOnOwnerDestroyed`
  (params (DestroyedActor :type "Actor Object Reference"))
  (for _array_element (`self.Items`)
    (`/Game/Blueprints/Storage/Items/BP_StorageItem.DestroyItem` _array_element)))

(fn `DropItemToWorld`
  (params (Item :type "/Game/Blueprints/Storage/Items/BP_StorageItem Object Reference") (Count :type Integer) (DropAll :type Boolean))
  (locals (L_Item :type "/Game/Blueprints/Storage/Items/BP_StorageItem Object Reference") (LCount :type Integer))
  (bind _actualitemscale (`/Game/Blueprints/Storage/Items/BP_StorageItem.ActualItemScale` (`local.L_Item`)))
  (bind _actualitemscale_2 (`/Game/Blueprints/Storage/Items/BP_StorageItem.ActualItemScale` (`local.L_Item`)))
  (`/Engine/EditorBlueprintResources/StandardMacros.IsValid` Item
    (:`Is Valid`
      (bind _output_get (set `local.L_Item` Item))
      (if DropAll
        ;[1 1 1] Drop all stack
        (bind _removed (`self.Remove Item` (`local.L_Item`) 0 false true :!label _label))
        (if _removed
          (bind _returnvalue (`|SpawnActorFromClass` (`GameplayStatics.GetObjectClass` (`local.L_Item`)) (`KismetMathLibrary.MakeTransform` (0.0 0.0 0.0) (struct) (select `bool` (== _actualitemscale_2 (0.0 0.0 0.0)) :`false` _actualitemscale_2 :`true` (1.0 1.0 1.0))) "AlwaysSpawn" "OverrideRootScale" null (`local.LCount`) null))
          (bind _dropped (`/Game/Blueprints/Storage/Items/BP_StorageItem.DroppedToWorld` _returnvalue (`self.DropLocation`)))
          (if _dropped
            (`Actor.K2_DestroyActor` (`local.L_Item`))))
        (else
          (set `local.LCount` Count)
          (if (`self.Is Full Stack by Count` _output_get (`local.LCount`))
            (goto _label)
            (else
              ;[1 1 1] Drop part of stack
              (bind _removed_2 (`self.Remove Item` (`local.L_Item`) (`local.LCount`)))
              (if _removed_2
                (bind _returnvalue_2 (`|SpawnActorFromClass` (`GameplayStatics.GetObjectClass` (`local.L_Item`)) (`KismetMathLibrary.MakeTransform` (0.0 0.0 0.0) (struct) (select `bool` (== _actualitemscale (0.0 0.0 0.0)) :`false` _actualitemscale :`true` (1.0 1.0 1.0))) "AlwaysSpawn" "OverrideRootScale" null (`local.LCount`) null))
                (`/Game/Blueprints/Storage/Items/BP_StorageItem.DroppedToWorld` _returnvalue_2 (`self.DropLocation`))))))))))

(fn `DropLocation`
  (returns (ReturnValue :type "Vector Structure"))
  (bind _returnvalue (`self.GetOwner`))
  (return (+ (`Actor.K2_GetActorLocation` _returnvalue) (* (`Actor.GetActorForwardVector` _returnvalue) (`self.DropDistance`)))))

(fn `GenerateRandomItems`
  (returns (Items :type "Array of /Game/Blueprints/Storage/ST_BeginItemInfo Structure"))
  (locals (L_GeneratedItems :type "Array of /Game/Blueprints/Storage/ST_BeginItemInfo Structure"))
  (for _array_element (`self.RandomBeginItems`)
    (bind (_iteminfo _chance) (break `/Game/Blueprints/Storage/ST_RandomItem` _array_element))
    (if (>= _chance (`KismetMathLibrary.RandomFloatInRange` 0.0 100.0))
      (`KismetArrayLibrary.Array_Add` (`local.L_GeneratedItems`) _iteminfo)))
  (return (`local.L_GeneratedItems`)))

(fn `Get Item in Storage by Class`
  (params (Class :type "/Game/Blueprints/Storage/Items/BP_StorageItem Class Reference"))
  (returns (Item :type "/Game/Blueprints/Storage/Items/BP_StorageItem Object Reference") (WasFound :type Boolean))
  (locals (L_Class :type "/Game/Blueprints/Storage/Items/BP_StorageItem Class Reference") (L_Item :type "/Game/Blueprints/Storage/Items/BP_StorageItem Object Reference") (L_ItemFound :type Boolean))
  (set `local.L_Class` Class)
  (for _array_element (`self.Items`)
    (if (== (`GameplayStatics.GetObjectClass` _array_element) (`local.L_Class`))
      (set `local.L_Item` _array_element)
      (set `local.L_ItemFound` true)
      (break)))
  (return (`local.L_Item`) (`local.L_ItemFound`)))

(fn `GetItems`
  (returns (Items :type "Array of /Game/Blueprints/Storage/Items/BP_StorageItem Object Reference"))
  (return (`self.Items`)))

(fn `GetWeight`
  (returns (Total :type "Float (double-precision)") (Max :type "Float (double-precision)"))
  (return (`self.StorageTotalWeight`) (`self.StorageMaxWeight`)))

(fn `Is Full Stack by Count`
  (params (Item :type "/Game/Blueprints/Storage/Items/BP_StorageItem Object Reference") (Count :type Integer))
  (returns (FullStack :type Boolean) (Remain :type Integer))
  (bind _returnvalue (- (`/Game/Blueprints/Storage/Items/BP_StorageItem.Count` Item) Count))
  (return (<= _returnvalue 0) _returnvalue))

(fn `Place to Another Storage`
  (params (Item :type "/Game/Blueprints/Storage/Items/BP_StorageItem Object Reference") (StorageIn :type "/Game/Blueprints/Storage/BP_StorageComponent Object Reference") (Count :type Integer) (Total :type Boolean :default true))
  (returns (Placed :type Boolean) (PlacedItem :type "/Game/Blueprints/Storage/Items/BP_StorageItem Object Reference"))
  (locals (L_Item :type "/Game/Blueprints/Storage/Items/BP_StorageItem Object Reference") (L_StorageIn :type "/Game/Blueprints/Storage/BP_StorageComponent Object Reference") (L_Count :type Integer) (L_Total :type Boolean :default true))
  (bind _l_item (`local.L_Item`))
  (bind _output_get (set `local.L_Item` Item))
  (bind _output_get_2 (set `local.L_StorageIn` StorageIn))
  (set `local.L_Count` Count)
  (bind _output_get_3 (set `local.L_Total` Total))
  (if _output_get_3
    ;[1 1 1] Place full items to another storage
    (bind _canbeadded (`self.CheckIfItemCanBeAdded` _output_get_2 _output_get))
    (if _canbeadded
      (bind _removed (`self.Remove Item` _l_item (`/Game/Blueprints/Storage/Items/BP_StorageItem.Count` _l_item) false true))
      (if _removed
        (bind _added (`self.Add Item` (`local.L_StorageIn`) (`local.L_Item`)))
        (if _added
          (return true (`local.L_Item`))
          (else
            (return false null)))
        (else
          (return false null)))
      (else
        (return false null)))
    (else
      ;[1 1 1] Place item to another storage by count
      (bind _createditems (`self.CreateItems` (`local.L_StorageIn`) (`|MakeArray` (make `/Game/Blueprints/Storage/ST_BeginItemInfo` (`GameplayStatics.GetObjectClass` (`local.L_Item`)) (`local.L_Count`)))))
      (if (> (`KismetArrayLibrary.Array_Length` _createditems) 0)
        (`self.Remove Item` (`local.L_Item`) (`local.L_Count`))
        (return true (`|GetArrayItem` _createditems))
        (else
          (return false null))))))

(fn `Remove Item`
  (params (StorageItem :type "/Game/Blueprints/Storage/Items/BP_StorageItem Object Reference") (Count :type Integer) (DestroyAfterLast :type Boolean) (RemoveAll :type Boolean))
  (returns (Removed :type Boolean))
  (locals (L_Item :type "/Game/Blueprints/Storage/Items/BP_StorageItem Object Reference") (L_Count :type Integer) (LRemoveAllStackedItem :type Boolean :default false) (L_Destroy :type Boolean))
  (bind _returnvalue (> (`local.L_Count`) 0))
  (`/Engine/EditorBlueprintResources/StandardMacros.IsValid` StorageItem
    (:`Is Valid`
      (bind _output_get (set `local.L_Item` StorageItem))
      (set `local.L_Destroy` DestroyAfterLast)
      (set `local.L_Count` (`KismetMathLibrary.SelectInt` (`/Game/Blueprints/Storage/Items/BP_StorageItem.Count` _output_get) Count RemoveAll))
      (if (== (`.Storage` (`/Game/Blueprints/Storage/Items/BP_StorageItem.IsInStorage` (`local.L_Item`))) self)
        (bind _removedall (`self.Remove Stacked Item` (`local.L_Item`) (`local.L_Count`)))
        (set `local.LRemoveAllStackedItem` _removedall)
        (`self.ChangeTotalWeight` (* -1 (`/Game/Blueprints/Storage/Items/BP_StorageItem.GetTotalWeight` (`local.L_Item`) _removedall (`local.L_Count`))))
        (if (`local.LRemoveAllStackedItem`)
          (`KismetArrayLibrary.Array_RemoveItem` (`self.Items`) (`local.L_Item`))
          (`/Game/Blueprints/Storage/Items/BP_StorageItem.ItemRemovedFromStorage` (`local.L_Item`) self)
          (if (`local.L_Destroy`)
            (`/Game/Blueprints/Storage/Items/BP_StorageItem.DestroyItem` (`local.L_Item`))
            (`self.InventoryUpdated`)
            (return true)
            (else
              (`self.InventoryUpdated`)
              (return true)))
          (else
            (if _returnvalue
              (`self.InventoryUpdated`))
            (return _returnvalue)))
        (else
          (return false))))))

(fn `Remove Stacked Item`
  (params (Item :type "/Game/Blueprints/Storage/Items/BP_StorageItem Object Reference") (Count :type Integer))
  (returns (RemovedAll :type Boolean))
  (locals (L_Item :type "/Game/Blueprints/Storage/Items/BP_StorageItem Object Reference") (L_inCount :type Integer) (L_RemovedAll :type Boolean))
  (bind _l_item (`local.L_Item`))
  (bind (_fullstack _remain) (`self.Is Full Stack by Count` (`local.L_Item`) (`local.L_inCount`)))
  (set `local.L_Item` Item)
  (set `local.L_inCount` Count)
  (bind _output_get (set `local.L_RemovedAll` _fullstack))
  (if (not _output_get)
    (set `/Game/Blueprints/Storage/Items/BP_StorageItem.Count` _remain _l_item))
  (`/Game/Blueprints/Storage/Items/BP_StorageItem.ItemRemoved-BP_StorageItem` _l_item _l_item (`local.L_inCount`))
  (return (`local.L_RemovedAll`)))

(fn `StackItem`
  (params (Item :type "/Game/Blueprints/Storage/Items/BP_StorageItem Object Reference") (StorageItem :type "/Game/Blueprints/Storage/Items/BP_StorageItem Object Reference"))
  (locals (l_item :type "/Game/Blueprints/Storage/Items/BP_StorageItem Object Reference") (L_StackIn :type "/Game/Blueprints/Storage/Items/BP_StorageItem Object Reference"))
  (set `local.l_item` Item)
  (set `local.L_StackIn` StorageItem)
  (set `/Game/Blueprints/Storage/Items/BP_StorageItem.Count` (+ (`/Game/Blueprints/Storage/Items/BP_StorageItem.Count` (`local.l_item`)) (`/Game/Blueprints/Storage/Items/BP_StorageItem.Count` (`local.L_StackIn`))) (`local.L_StackIn`))
  (`self.ChangeTotalWeight` (`/Game/Blueprints/Storage/Items/BP_StorageItem.GetTotalWeight` (`local.l_item`) true 0)))