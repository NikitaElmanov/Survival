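; BP_BranchWeapon is an equippable tree-branch melee weapon, built on a parent weapon Blueprint.
; Equipping turns off the Branch component's collision and unequipping restores query and physics collision, each alongside the parent logic.
; UseWeapon defers to the parent and, when the use succeeds, calls TraceHit with an angle, radius and trace count to detect hits around the swing.
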(fn `EquipItem`
  (params (EquipToCharacter :type "/Game/Blueprints/Characters/SurvivalCharacter Object Reference"))
  (returns (Equiped :type Boolean))
  (bind _equiped (`parent.EquipItem` EquipToCharacter))
  (`PrimitiveComponent.SetCollisionEnabled` (`self.branch`) "NoCollision")
  (return _equiped))

(fn `UnEquipItem`
  (returns (UnEquiped :type Boolean))
  (bind _unequiped (`parent.UnEquipItem`))
  (`PrimitiveComponent.SetCollisionEnabled` (`self.branch`) "QueryAndPhysics")
  (return _unequiped))

(fn `UserConstructionScript`
  (`parent.UserConstructionScript`))

(fn `UseWeapon`
  (params (Use :type Boolean))
  (returns (Used :type Boolean) (Weapon :type "/Game/Blueprints/Storage/Items/Equipables/Weapons/Weapon Object Reference"))
  (locals (L_Weapon :type "/Game/Blueprints/Storage/Items/Equipables/Weapons/Weapon Object Reference"))
  (bind (_used _weapon) (`parent.UseWeapon` Use))
  (set `local.L_Weapon` _weapon)
  (if _used
    (`self.TraceHit` 45.0 100.0 20)
    (return true (`local.L_Weapon`))
    (else
      (return false (`local.L_Weapon`)))))