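; BP_Pickaxe is an equipable pickaxe weapon that strikes with a short-range sphere trace.
; It overrides UseWeapon, calling the parent first and running SphereTraceHit only when the parent reports the weapon was used.
; A successful hit calls PlaySlashSound, which starts SlashAudio unless it is already playing.
; The event graph holds only disabled default events.
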(fn `PlaySlashSound`
  (if (not (`AudioComponent.IsPlaying` (`self.SlashAudio`)))
    (`AudioComponent.Play` (`self.SlashAudio`) 0.0)))

(fn `UserConstructionScript`
  (`parent.UserConstructionScript`))

(fn `UseWeapon`
  (params (Use :type Boolean) (asMelee :type Boolean))
  (returns (Used :type Boolean) (Weapon :type "/Game/Blueprints/Storage/Items/Equipables/Weapons/Weapon Object Reference"))
  (locals (L_Weapon :type "/Game/Blueprints/Storage/Items/Equipables/Weapons/Weapon Object Reference"))
  (bind (_used _weapon) (`parent.UseWeapon` Use asMelee))
  (if _used
    (set `local.L_Weapon` _weapon)
    (bind _damaged (`self.SphereTraceHit` 150.0 50.0))
    (if _damaged
      (`self.PlaySlashSound`))
    (return true (`local.L_Weapon`))))