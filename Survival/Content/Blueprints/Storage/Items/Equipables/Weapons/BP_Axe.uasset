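; BP_Axe is an equipable melee axe weapon, a child Blueprint of a weapon base class.
; It overrides UseWeapon, calling the parent first and, when that reports a successful use, running a short sphere trace hit before returning the used weapon.
; The event graph and construction script add no logic of their own.
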(fn `UserConstructionScript`
  (`parent.UserConstructionScript`))

(fn `UseWeapon`
  (params (Use :type Boolean))
  (returns (Used :type Boolean) (Weapon :type "/Game/Blueprints/Storage/Items/Equipables/Weapons/Weapon Object Reference"))
  (locals (L_Weapon :type "/Game/Blueprints/Storage/Items/Equipables/Weapons/Weapon Object Reference"))
  (bind (_used _weapon) (`parent.UseWeapon` Use))
  (if _used
    (set `local.L_Weapon` _weapon)
    (`self.SphereTraceHit` 150.0 20.0)
    (return true (`local.L_Weapon`))))