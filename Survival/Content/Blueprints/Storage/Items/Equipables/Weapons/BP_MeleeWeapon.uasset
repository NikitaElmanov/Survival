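; Melee weapon Blueprint that gates the parent UseWeapon on IsAbleToUseWeapon and provides three ways to damage targets in front of the wielder.
; SphereTraceHit sweeps a sphere along the pitch-adjusted aim, choosing its trace channel by whether the player is the instigator.
; TraceHit fans line traces across an angle, damaging each unique actor found.
; ConeOverlapHit damages actors overlapping a spawned, scaled mesh component, with its filtering and cleanup nodes left disconnected.
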(fn `ConeOverlapHit`
  (params (Radius :type "Float (double-precision)") (Angle :type "Float (double-precision)") (Height :type "Float (double-precision)"))
  (locals (L_Collision :type "StaticMeshComponent Object Reference") (L_ActorsCollision :type "Array of Actor Object Reference") (L_Hit :type "StaticMeshComponent Object Reference") (L_ActorLocation :type "Vector Structure" :default (0.0 0.0 0.0)) (L_ActorCollisionForIgnoring :type "Array of Actor Object Reference"))
  (bind _returnvalue (`self.K2_GetActorLocation` (`self.EquippedToCharacter`)))
  (set `local.L_ActorLocation` _returnvalue)
  (bind _returnvalue_2 (`AddComponent|NODE_AddStaticMeshComponent-0` :`bManualAttachment` true))
  (bind _output_get (set `local.L_Collision` _returnvalue_2))
  (`SceneComponent.K2_SetWorldTransform` _output_get (`KismetMathLibrary.MakeTransform` _returnvalue (`KismetMathLibrary.Conv_VectorToRotator` (`self.HitDirection_0`)) (`KismetMathLibrary.MakeVector` Radius (/ (+ Radius Angle) 2.0) Height)) false false)
  (bind _output_get_2 (set `local.L_ActorsCollision` (`PrimitiveComponent.GetOverlappingActors` (`local.L_Collision`) "/Script/Engine.Actor")))
  (for _ _output_get_2
    (`GameplayStatics.ApplyDamage` null (`self.Damage`) (`Pawn.GetController` (`self.GetInstigator`)) self)))

(fn `HitDirection_0`
  (returns (Out :type "Vector Structure"))
  (bind (_returnvalue_roll _returnvalue_pitch) (`KismetMathLibrary.BreakRotator` (`self.K2_GetActorRotation` (`Pawn.GetController` (`self.EquippedToCharacter`)))))
  (return (`KismetMathLibrary.RotateAngleAxis` (`self.GetActorForwardVector` (`self.EquippedToCharacter`)) (* -1 _returnvalue_pitch) (`self.GetActorRightVector` (`self.EquippedToCharacter`)))))

(fn `HitInitialLocation_0`
  (returns (Out :type "Vector Structure"))
  (return (+ (`self.K2_GetActorLocation` (`self.EquippedToCharacter`)) (0.0 0.0 50.0))))

(fn `SphereTraceHit`
  (params (CapsuleLength :type "Float (double-precision)") (SphereHitRadius :type "Float (double-precision)"))
  (returns (Damaged :type Boolean))
  (locals (L_CapsuleLength :type "Float (double-precision)") (L_SphereHitRadius :type "Float (double-precision)"))
  (bind _out (`self.HitInitialLocation_0`))
  (set `local.L_CapsuleLength` CapsuleLength)
  (set `local.L_SphereHitRadius` SphereHitRadius)
  (bind (_outhit _returnvalue) (`KismetSystemLibrary.SphereTraceSingle` _out (+ _out (* (`self.HitDirection_0`) (`local.L_CapsuleLength`))) (`local.L_SphereHitRadius`) (select `bool` (== (`self.GetInstigator`) (`GameplayStatics.GetPlayerPawn` 0)) :`false` "TraceTypeQuery4" :`true` "TraceTypeQuery1" :!type "ETraceTypeQuery Enum") false (`|MakeArray` (`self.EquippedToCharacter`) :!type "Actor Object Reference")))
  (if _returnvalue
    (bind _damaged (`self.DealDamage` (`self.Damage`) _outhit "NewEnumerator1" self))
    (return _damaged)))

(fn `TraceHit`
  (params (Angle :type "Float (double-precision)") (Radius :type "Float (double-precision)") (TraceNumber :type Integer))
  (locals (L_Angle :type "Float (double-precision)") (L_Radius :type "Float (double-precision)") (L_Actors :type "Array of Actor Object Reference") (L_HitResults :type "Array of HitResult Structure") (L_HitResult :type "HitResult Structure"))
  (bind _out (`self.HitInitialLocation_0`))
  (bind (_returnvalue_roll _returnvalue_pitch) (`KismetMathLibrary.BreakRotator` (`self.K2_GetActorRotation` (`Pawn.GetController` (`self.EquippedToCharacter`)))))
  (set `local.L_Angle` Angle)
  (set `local.L_Radius` Radius)
  (for _index (range TraceNumber)
    (bind (_outhit _returnvalue) (`KismetSystemLibrary.LineTraceSingle` :`Start` _out :`End` (+ _out (* (`KismetMathLibrary.RotateAngleAxis` (`KismetMathLibrary.GreaterGreater_VectorRotator` (`self.GetActorForwardVector` (`self.EquippedToCharacter`)) (`KismetMathLibrary.MakeRotator` 0.0 0.0 (+ (* _index (/ (`local.L_Angle`) (`KismetMathLibrary.Conv_IntToDouble` TraceNumber))) (* -1 (/ (`local.L_Angle`) 2.0))))) (* -1 _returnvalue_pitch) (`self.GetActorRightVector` (`self.EquippedToCharacter`))) (`local.L_Radius`))) :`TraceChannel` "TraceTypeQuery1" :`DrawDebugType` "ForDuration"))
    (if _returnvalue
      (bind _output_get (set `local.L_HitResult` _outhit))
      (bind (_bblockinghit _binitialoverlap _time _distance _location _impactpoint _normal _impactnormal _physmat _hitactor) (`GameplayStatics.BreakHitResult` _output_get))
      (if (not (>= (`KismetArrayLibrary.Array_Find` (`local.L_Actors`) _hitactor) 0))
        (`KismetArrayLibrary.Array_Add` (`local.L_Actors`) _hitactor)
        (`KismetArrayLibrary.Array_Add` (`local.L_HitResults`) (`local.L_HitResult`)))))
  (for _array_element (`local.L_HitResults`)
    (`self.DealDamage` (`self.Damage`) _array_element "NewEnumerator0" self)))

(fn `UserConstructionScript`
  (`parent.UserConstructionScript`))

(fn `UseWeapon`
  (params (Use :type Boolean) (asMelee :type Boolean))
  (returns (Used :type Boolean) (Weapon :type "/Game/Blueprints/Storage/Items/Equipables/Weapons/Weapon Object Reference"))
  (if Use
    (if (`self.IsAbleToUseWeapon`)
      (bind (_used _weapon) (`parent.UseWeapon` true asMelee))
      (return _used _weapon)
      (else
        (bind (_used_2 _weapon_2) (`parent.UseWeapon` false asMelee))
        (return _used_2 _weapon_2)))
    (else
      (bind (_used_3 _weapon_3) (`parent.UseWeapon` false asMelee))
      (return _used_3 _weapon_3))))