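; Cylinder hat equipable clothing item that boosts the wearer's jump while equipped.
; It overrides the parent's equip-modifier add and remove functions, which gate the change on the parent call succeeding.
; On success it raises or lowers the character movement's JumpZVelocity by a fixed amount and reports the result.
; The event graph holds only disabled default events.
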(fn `AddEquipModifierToOwner`
  (returns (Added :type Boolean))
  (bind _added (`parent.AddEquipModifierToOwner`))
  (if _added
    (set `CharacterMovementComponent.JumpZVelocity` (+ (`CharacterMovementComponent.JumpZVelocity` (`Character.CharacterMovement` (`self.EquippedToCharacter`))) 300.0) (`Character.CharacterMovement` (`self.EquippedToCharacter`)))
    (return true)
    (else
      (return false))))

(fn `RemoveModifierFromOwner`
  (returns (Removed :type Boolean))
  (bind _removed (`parent.RemoveModifierFromOwner`))
  (if _removed
    (set `CharacterMovementComponent.JumpZVelocity` (- (`CharacterMovementComponent.JumpZVelocity` (`Character.CharacterMovement` (`self.EquippedToCharacter`))) 300.0) (`Character.CharacterMovement` (`self.EquippedToCharacter`)))
    (return true)
    (else
      (return false))))

(fn `UserConstructionScript`
  (`parent.UserConstructionScript`))