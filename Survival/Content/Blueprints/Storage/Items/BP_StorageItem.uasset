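; Base actor for an item that characters pick up via Interact into their storage component, with stack count, weight and a breakable condition.
; When stored, it stays alive, frozen and teleported below the world, taking owner and Instigator from the storage's owner.
; Dropping teleports it back and re-enables physics on its meshes, which freezing snaps to the root.
; Removal delegates to the owning storage; use and crafting hooks are stubs.
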(fn `ChangeCondition`
  (params (Value :type "Float (double-precision)"))
  (returns (Broken :type Boolean))
  (bind _output_get (set `self.Condition` (+ Value (`self.Condition`))))
  (if (<= _output_get 0.0)
    (set `self.Broken` true)
    (`self.ItemBroken` self)
    (return true)
    (else
      (return false))))

(fn `Crafted`)

(fn `DestroyItem`
  (`self.K2_DestroyActor`))

(fn `DroppedToWorld`
  (params (Location :type "Vector Structure"))
  (returns (Dropped :type Boolean))
  (`self.Freeze Physics Components` true)
  (`self.K2_SetActorLocation` Location false true)
  (`self.SetActorHiddenInGame` false)
  (`self.Freeze Physics Components` false)
  (return true))

(fn `Freeze Physics Components`
  (params (Freeze :type Boolean))
  (locals (L_Freeze :type Boolean) (L_SkeletalMC :type "SkeletalMeshComponent Object Reference"))
  (bind _l_freeze (`local.L_Freeze`))
  (set `local.L_Freeze` Freeze)
  (for _array_element (`self.Components`)
    (bind _asskeletal_mesh_component (cast `SkeletalMeshComponent` _array_element)
      (:`then`
        ;[1 1 1] SkeletalMeshComponent peek/drop
        (bind _output_get (set `local.L_SkeletalMC` _asskeletal_mesh_component))
        (`PrimitiveComponent.SetSimulatePhysics` _output_get (not _l_freeze))
        (`PrimitiveComponent.SetCollisionEnabled` (`local.L_SkeletalMC`) (select `bool` _l_freeze :`false` "QueryAndPhysics" :`true` "NoCollision" :!type "ECollisionEnabled Enum"))
        (if (`local.L_Freeze`)
          (`SceneComponent.K2_AttachToComponent` (`local.L_SkeletalMC`) (`self.DefaultSceneRoot`) "None" "SnapToTarget" "SnapToTarget" "SnapToTarget" true)))
      (:`CastFailed`
        ;[1 1 1] MeshComponent peek/drop
        (bind _asmesh_component (cast `MeshComponent` _array_element))
        (`PrimitiveComponent.SetSimulatePhysics` _asmesh_component (not (`local.L_Freeze`)))
        (if (`local.L_Freeze`)
          (`SceneComponent.K2_AttachToComponent` _asmesh_component (`self.DefaultSceneRoot`) "None" "SnapToTarget" "SnapToTarget" "SnapToTarget" true))))))

(fn `GetInstigatorPlayerController`
  (returns (PlayerController :type "PlayerController Object Reference"))
  (bind _asplayer_controller (cast `PlayerController` (`self.GetInstigatorController`))
    (:`then`
      (return _asplayer_controller))
    (:`CastFailed`
      (return null))))

(fn `GetTotalWeight`
  (params (Total :type Boolean) (InCount :type Integer))
  (returns (Weight :type "Float (double-precision)"))
  (locals (NewLocalVar_0 :type "Float (double-precision)" :default 0.0))
  (return (* (`KismetMathLibrary.SelectInt` (`self.Count`) InCount Total) (`self.Weight`))))

(fn `Interact`
  (params (Character :type "/Game/Blueprints/Characters/SurvivalCharacter Object Reference"))
  (returns (Successfull :type Boolean) (Message :type String))
  (bind _added (`/Game/Blueprints/Storage/BP_StorageComponent.Add Item` (`/Game/Blueprints/Characters/SurvivalCharacter.BP_StorageComponent` Character) self))
  (return _added (`KismetMathLibrary.SelectString` "item added" "you don't have enogh place" _added)))

(fn `IsInStorage`
  (returns (InStorage :type Boolean) (Storage :type "/Game/Blueprints/Storage/BP_StorageComponent Object Reference"))
  (return (`self.InStorage`) (`self.OwningStorage`)))

(fn `Item Added to Storage`
  (params (Storage :type "/Game/Blueprints/Storage/BP_StorageComponent Object Reference"))
  (set `self.OwningStorage` Storage)
  (set `self.InStorage` true)
  (`self.Freeze Physics Components` true)
  (`self.K2_SetActorLocation` (0.0 0.0 -1000.0) false true)
  (`self.SetActorHiddenInGame` false)
  (`|ExecutionSequence`
    (:`then_0`
      ;[1 1 1] Set up instigator
      (bind _aspawn (cast `Pawn` (`ActorComponent.GetOwner` (`self.OwningStorage`))))
      (set `self.Instigator` _aspawn))
    (:`then_1`
      ;[1 1 1] Set up owner
      (`self.SetOwner` (`ActorComponent.GetOwner` (`self.OwningStorage`))))))

(fn `ItemRemovedFromStorage`
  (params (FromStorage :type "/Game/Blueprints/Storage/BP_StorageComponent Object Reference"))
  (set `self.OwningStorage` null)
  (set `self.InStorage` false)
  (`self.SetOwner` null)
  (set `self.Instigator` null))

(fn `RemoveItem`
  (params (Count :type Integer))
  (locals (L_Count :type Integer))
  (bind (_instorage _storage) (`self.IsInStorage`))
  (set `local.L_Count` Count)
  (if _instorage
    (`/Game/Blueprints/Storage/BP_StorageComponent.RemoveItem` _storage false self (`local.L_Count`) false)
    (`self.ItemRemoved` self (`local.L_Count`))
    (else
      (bind _output_get (set `self.Count` (- (`self.Count`) (`local.L_Count`))))
      (if (<= _output_get 0)
        (`self.ItemRemoved` self (`local.L_Count`))
        (`self.DestroyItem`)))))

(fn `UsedToCraft`)

(fn `UseItem`
  (returns (Used :type Boolean))
  (return false))

(fn `UserConstructionScript`
  (set `self.Components` (`SceneComponent.GetChildrenComponents` (`self.DefaultSceneRoot`) true)))