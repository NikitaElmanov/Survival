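; Crafting component that matches held items, by class and count, against recipes in the RecipesData table and crafts the result.
; Find functions look up recipes from items or items for a recipe, though FindAllRecipesByItems returns every row once any matches.
; Craft notifies and deducts the ingredients, then spawns the result hidden and physics-frozen at a fixed location.
; Convert and its reverse lookup by output item are unfinished stubs.
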(fn `Convert`
  (params (Item :type "/Game/Blueprints/Storage/Items/BP_StorageItem Object Reference"))
  (locals (L_Recipe :type "/Game/Blueprints/Recipes/ST_CraftRecipe Structure"))
  (bind (_recipefound _recipe) (`self.FindConvertRecipeByItem` Item))
  (bind _output_get (set `local.L_Recipe` _recipe))
  (if _recipefound
    (for _ (`.Items_6_96ECA29D406BC79F1839DDA5CEA551BB` (break `/Game/Blueprints/Recipes/ST_CraftRecipe` _output_get))
      _)))

(fn `Craft`
  (params (Items :type "Array of /Game/Blueprints/Storage/Items/BP_StorageItem Object Reference") (Recipe :type "/Game/Blueprints/Recipes/ST_CraftRecipe Structure"))
  (returns (CraftedItem :type "/Game/Blueprints/Storage/Items/BP_StorageItem Object Reference"))
  (locals (L_Items :type "Array of /Game/Blueprints/Storage/Items/BP_StorageItem Object Reference") (L_Recipe :type "/Game/Blueprints/Recipes/ST_CraftRecipe Structure") (NewLocalVar_0 :type "/Game/Blueprints/Storage/ST_BeginItemInfo Structure"))
  (bind (_item _count) (break `/Game/Blueprints/Storage/ST_BeginItemInfo` (`.Item_7_70C275B74D28336D276835B9BCF7CC99` (break `/Game/Blueprints/Recipes/ST_CraftRecipe` (`local.L_Recipe`)))))
  (set `local.L_Items` Items)
  (set `local.L_Recipe` Recipe)
  (`|ExecutionSequence`
    (:`then_0`
      (for _array_element (`local.L_Items`)
        (`/Game/Blueprints/Storage/Items/BP_StorageItem.UsedToCraft` _array_element))
      (`self.RemoveCraftedItems` (`local.L_Items`) (`.Items_6_96ECA29D406BC79F1839DDA5CEA551BB` (break `/Game/Blueprints/Recipes/ST_CraftRecipe` (`local.L_Recipe`)))))
    (:`then_1`
      (bind _returnvalue (`|SpawnActorFromClass` _item (`KismetMathLibrary.MakeTransform` (700.0 700.0 700.0)) "AlwaysSpawn" "OverrideRootScale" null _count null))
      (`/Game/Blueprints/Storage/Items/BP_StorageItem.Freeze Physics Components` _returnvalue true)
      (`Actor.SetActorHiddenInGame` _returnvalue true)
      (`/Game/Blueprints/Storage/Items/BP_StorageItem.Crafted` _returnvalue)
      (return _returnvalue))))

(fn `FindAllRecipesByItems`
  (params (Items :type "Array of /Game/Blueprints/Storage/Items/BP_StorageItem Object Reference"))
  (returns (Recipes :type "Array of /Game/Blueprints/Recipes/ST_CraftRecipe Structure") (RecipeFound :type Boolean))
  (locals (L_Items :type "Array of /Game/Blueprints/Storage/Items/BP_StorageItem Object Reference") (L_Recipe :type "Array of /Game/Blueprints/Recipes/ST_CraftRecipe Structure") (L_AnyRecipeWasFound :type Boolean) (L_NeededItemInfoClass :type "/Game/Blueprints/Storage/Items/BP_StorageItem Class Reference") (L_NeededItemInfoCount :type Integer) (L_ItemsForRecipeWasFound :type Boolean) (L_NeededItemFound :type Boolean))
  (bind _l_recipe (`local.L_Recipe`))
  (bind _l_anyrecipewasfound (`local.L_AnyRecipeWasFound`))
  (set `local.L_Items` Items)
  (bind _outrownames (`DataTableFunctionLibrary.GetDataTableRowNames` (`self.RecipesData`)))
  (for _array_element _outrownames
    (bind _returnvalue (`|GetDataTableRow` (`self.RecipesData`) _array_element)
      (:`then`
        (`KismetArrayLibrary.Array_Add` _l_recipe _returnvalue)
        (for _array_element_2 (`.Items_6_96ECA29D406BC79F1839DDA5CEA551BB` (break `/Game/Blueprints/Recipes/ST_CraftRecipe` _returnvalue))
          (bind (_item _count) (break `/Game/Blueprints/Storage/ST_BeginItemInfo` _array_element_2))
          (set `local.L_NeededItemInfoClass` _item)
          (set `local.L_NeededItemInfoCount` _count)
          (for _array_element_3 (`local.L_Items`)
            (if (and (== (`GameplayStatics.GetObjectClass` _array_element_3) (`local.L_NeededItemInfoClass`)) (>= (`/Game/Blueprints/Storage/Items/BP_StorageItem.Count` _array_element_3) (`local.L_NeededItemInfoCount`)))
              (set `local.L_NeededItemFound` true)
              (break)
              (else
                (set `local.L_NeededItemFound` false))))
          (if (`local.L_NeededItemFound`)
            (set `local.L_ItemsForRecipeWasFound` true)
            (else
              (set `local.L_ItemsForRecipeWasFound` false)
              (break))))
        (if (`local.L_ItemsForRecipeWasFound`)
          (set `local.L_AnyRecipeWasFound` true)))))
  (if (not _l_anyrecipewasfound)
    (`KismetArrayLibrary.Array_Clear` (`local.L_Recipe`)))
  (return _l_recipe _l_anyrecipewasfound))

(fn `FindConvertRecipeByItem`
  (params (Item :type "/Game/Blueprints/Storage/Items/BP_StorageItem Object Reference"))
  (returns (RecipeFound :type Boolean) (Recipe :type "/Game/Blueprints/Recipes/ST_CraftRecipe Structure"))
  (locals (L_Item :type "/Game/Blueprints/Storage/Items/BP_StorageItem Object Reference") (L_Recipe :type "/Game/Blueprints/Recipes/ST_CraftRecipe Structure") (L_RecipeFound :type Boolean))
  (set `local.L_Item` Item)
  (bind _outrownames (`DataTableFunctionLibrary.GetDataTableRowNames` (`self.RecipesData`)))
  (for _array_element _outrownames
    (bind _returnvalue (`|GetDataTableRow` (`self.RecipesData`) _array_element)
      (:`then`
        (if (== (`.Item_13_A53D5A4948F713A82DCFFC95F9D7867E` (break `/Game/Blueprints/Storage/ST_BeginItemInfo` (`.Item_7_70C275B74D28336D276835B9BCF7CC99` (break `/Game/Blueprints/Recipes/ST_CraftRecipe` _returnvalue)))) (`GameplayStatics.GetObjectClass` (`local.L_Item`)))
          (return (`local.L_RecipeFound`) (`local.L_Recipe`))))))
  (return false))

(fn `FindItemsByRecipe`
  (params (Resipe :type "/Game/Blueprints/Recipes/ST_CraftRecipe Structure") (InItem :type "Array of /Game/Blueprints/Storage/Items/BP_StorageItem Object Reference"))
  (returns (NeededItemsFound :type Boolean) (Items :type "Array of /Game/Blueprints/Storage/Items/BP_StorageItem Object Reference"))
  (locals (L_NeededCountItems :type Integer) (L_Found :type Boolean :default true) (L_Items :type "Array of /Game/Blueprints/Storage/Items/BP_StorageItem Object Reference") (L_FoundItem :type "/Game/Blueprints/Storage/Items/BP_StorageItem Object Reference") (L_InItems :type "Array of /Game/Blueprints/Storage/Items/BP_StorageItem Object Reference"))
  (set `local.L_InItems` InItem)
  (for _array_element (`.Items_6_96ECA29D406BC79F1839DDA5CEA551BB` (break `/Game/Blueprints/Recipes/ST_CraftRecipe` Resipe))
    (for _array_element_2 (`local.L_InItems`)
      (bind (_item _count) (break `/Game/Blueprints/Storage/ST_BeginItemInfo` _array_element))
      (set `local.L_NeededCountItems` _count)
      (if (== (`GameplayStatics.GetObjectClass` _array_element_2) _item)
        (bind _output_get (set `local.L_FoundItem` _array_element_2))
        (`/Engine/EditorBlueprintResources/StandardMacros.IsValid` _output_get
          (:`Is Valid`
            (if (< (`/Game/Blueprints/Storage/Items/BP_StorageItem.Count` _output_get) (`local.L_NeededCountItems`))
              (set `local.L_Found` false)
              (else
                (`KismetArrayLibrary.Array_Add` (`local.L_Items`) (`local.L_FoundItem`))
                (set `local.L_Found` true)
                (break)))))))
    (if (not (`local.L_Found`))
      (return false (`|MakeArray` null :!type "/Game/Blueprints/Storage/Items/BP_StorageItem Object Reference"))))
  (return true (`local.L_Items`)))

(fn `FindRecipeByItems`
  (params (Items :type "Array of /Game/Blueprints/Storage/Items/BP_StorageItem Object Reference"))
  (returns (Recipe :type "/Game/Blueprints/Recipes/ST_CraftRecipe Structure") (RecipeFound :type Boolean))
  (locals (L_Items :type "Array of /Game/Blueprints/Storage/Items/BP_StorageItem Object Reference") (L_Recipe :type "/Game/Blueprints/Recipes/ST_CraftRecipe Structure") (L_RecipeWasFound :type Boolean) (L_NeededItemInfoClass :type "/Game/Blueprints/Storage/Items/BP_StorageItem Class Reference") (L_NeededItemInfoCount :type Integer) (L_ItemsForRecipeWasFound :type Boolean) (L_NeededItemFound :type Boolean))
  (bind _l_recipewasfound (`local.L_RecipeWasFound`))
  (set `local.L_Items` Items)
  (bind _outrownames (`DataTableFunctionLibrary.GetDataTableRowNames` (`self.RecipesData`)))
  (for _array_element _outrownames
    (bind _returnvalue (`|GetDataTableRow` (`self.RecipesData`) _array_element)
      (:`then`
        (bind _output_get (set `local.L_Recipe` _returnvalue))
        (for _array_element_2 (`.Items_6_96ECA29D406BC79F1839DDA5CEA551BB` (break `/Game/Blueprints/Recipes/ST_CraftRecipe` _output_get))
          (bind (_item _count) (break `/Game/Blueprints/Storage/ST_BeginItemInfo` _array_element_2))
          (set `local.L_NeededItemInfoClass` _item)
          (set `local.L_NeededItemInfoCount` _count)
          (for _array_element_3 (`local.L_Items`)
            (if (and (== (`GameplayStatics.GetObjectClass` _array_element_3) (`local.L_NeededItemInfoClass`)) (>= (`/Game/Blueprints/Storage/Items/BP_StorageItem.Count` _array_element_3) (`local.L_NeededItemInfoCount`)))
              (set `local.L_NeededItemFound` true)
              (break)
              (else
                (set `local.L_NeededItemFound` false))))
          (if (`local.L_NeededItemFound`)
            (set `local.L_ItemsForRecipeWasFound` true)
            (else
              (set `local.L_ItemsForRecipeWasFound` false)
              (break))))
        (if (`local.L_ItemsForRecipeWasFound`)
          (set `local.L_RecipeWasFound` true)
          (break)
          (else
            (set `local.L_RecipeWasFound` false))))))
  (if (not _l_recipewasfound)
    (set `local.L_Recipe` (struct)))
  (return (`local.L_Recipe`) _l_recipewasfound))

(fn `RemoveCraftedItems`
  (params (Items :type "Array of /Game/Blueprints/Storage/Items/BP_StorageItem Object Reference") (NeededItems :type "Array of /Game/Blueprints/Storage/ST_BeginItemInfo Structure"))
  (locals (L_Item :type "/Game/Blueprints/Storage/Items/BP_StorageItem Object Reference"))
  (for _array_element Items
    (set `local.L_Item` _array_element)
    (for _array_element_2 NeededItems
      (bind (_item _count) (break `/Game/Blueprints/Storage/ST_BeginItemInfo` _array_element_2))
      (if (== (`GameplayStatics.GetObjectClass` (`local.L_Item`)) _item)
        (`/Game/Blueprints/Storage/Items/BP_StorageItem.RemoveItem` (`local.L_Item`) _count)))))