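; BP_RPGStats tracks RPG character progression through level, experience and the experience required for the next level.
; ChangeExperience feeds a threshold check that raises the level by one, calls CallNextLevel and recalculates the requirement through a rounded math expression.
; The check runs once per experience change, so a large gain grants only one level.
; Tick prints all three stats on screen every frame as colored debug text.
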(event EventBeginPlay)

(event EventTick
  (params (DeltaSeconds :type Float%20%28single-precision%29))
  (CallFunction|PrintPRGStats))

(fn ChangeExperience
  (params (Experience :type Float%20%28single-precision%29))
  (Variables|Default|SetExperience (+ Experience (Variables|Default|GetExperience)))
  (CallFunction|CheckExpforLevel))

(fn ChangeLevel
  (params (Level :type Integer))
  (Variables|Default|SetLevel (+ Level (Variables|Default|GetLevel))))

(fn CheckExpforLevel
  (if (>= (Variables|Default|GetExperience) (Variables|Default|GetExpForNextLevel))
    (CallFunction|ChangeLevel 1)
    (Default|CallNextLevel)
    (Variables|Default|SetExpForNextLevel (CallFunction|CalculateExpforCurrentLevel))))

(fn CalculateExpforCurrentLevel
  (return (Math|Conversions|ToFloat(Integer) (|((round({1029526C-416C-9B6E-407B-C1ABC1B2157F}))+({656A92A2-4518-B1EC-D0C0-D98E32A425AE}*100))))))

(fn PrintPRGStats
  (Utilities|FlowControl|Sequence
    (:then_0
      (Development|PrintString (Utilities|String|Append "Level: " (Utilities|String|ToString(Integer) (Variables|Default|GetLevel))) true true "(R=0.000000,G=0.225029,B=0.854167,A=1.000000)" 0.0))
    (:then_1
      (Development|PrintString (Utilities|String|Append "Exp: " (Utilities|String|ToString(Float) (Variables|Default|GetExperience))) true true "(R=0.854167,G=0.224196,B=0.606214,A=1.000000)" 0.0))
    (:then_2
      (Development|PrintString (Utilities|String|Append "ExpForNextL" (Utilities|String|ToString(Float) (Variables|Default|GetExpForNextLevel))) true true "(R=0.459956,G=0.854167,B=0.000000,A=1.000000)" 0.0))))