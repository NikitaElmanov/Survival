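; SurvivalCharacter is a survival character base that handles damage, death and sprint eligibility through a health stats component.
; Incoming damage is scaled down by armor, and depleted health triggers death: input off, ragdoll, a death notification and delayed destruction.
; Sprinting requires stamina while neither crouched nor falling.
; Height-based fall damage records takeoff location, but its landing calculation is disconnected and never runs.
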(event `self.ReceiveAnyDamage`
  (params (Damage :type "Float (single-precision)") (DamageType :type "DamageType Object Reference") (InstigatedBy :type "Controller Object Reference") (DamageCauser :type "Actor Object Reference"))
  ;[1 0.1927 0.1927] Get damage
  (`/Game/Blueprints/Characters/BP_HealthStats.ChangeHealth` (`self.BP_HealthStats`) (* (/ Damage (/ (+ (`self.ArmorValue`) 20.0) 20.0)) -1.0)))

(event `self.BP_HealthStats.HealthEnd`
  (params (Player :type "/Game/Blueprints/Characters/SurvivalCharacter Object Reference"))
  ;[1 1 1] Death
  (`self.Death`))

(event `self.OnJumped`
  ;[1 1 1] Fall Damage
  (set `self.LocationCharacter` (`self.K2_GetActorLocation`) :!label _label))

(event `self.OnWalkingOffLedge`
  (params (PreviousFloorImpactNormal :type "Vector Structure (by ref)") (PreviousFloorContactNormal :type "Vector Structure (by ref)") (PreviousLocation :type "Vector Structure (by ref)") (TimeDelta :type "Float (single-precision)"))
  ;[1 1 1] Fall Damage
  (goto _label))

(event `self.OnLanded`
  (params (Hit :type "HitResult Structure (by ref)"))
  ;[1 1 1] Fall Damage
)

(fn `CanSprint`
  (returns (canSprint :type Boolean))
  (return (and (> (`/Game/Blueprints/Characters/BP_HealthStats.Stamina` (`self.BP_HealthStats`)) 0.0) (not (`self.IsCrouching`)) (not (`|EnumEquality` (`CharacterMovementComponent.MovementMode` (`self.CharacterMovement`)) "MOVE_Falling")))))

(fn `Death`
  (set `self.Dead` true)
  (`self.DisableInput` (`GameplayStatics.GetPlayerController` 0))
  (`self.EnableRagdoll`)
  (`self.AnyCharacterDead-SurvivalCharacter` self)
  (`self.SetLifeSpan` (`self.DeathDestroyDelay`)))

(fn `EnableRagdoll`
  (returns (Enabled :type Boolean))
  (`PrimitiveComponent.SetCollisionEnabled` (`self.CapsuleComponent`) "NoCollision")
  (`PrimitiveComponent.SetSimulatePhysics` (`self.Mesh`) true)
  (`PrimitiveComponent.SetCollisionEnabled` (`self.Mesh`) "QueryAndPhysics")
  (`PrimitiveComponent.SetCollisionResponseToAllChannels` (`self.Mesh`) "ECR_Block")
  (`PrimitiveComponent.SetCollisionResponseToChannel` (`self.Mesh`) "ECC_Pawn" "ECR_Ignore")
  (return true))

(fn `GetInteractionInfo`
  (params (Distance :type "Float (double-precision)"))
  (returns (Hit :type "HitResult Structure"))
  (locals (NewLocalVar_0 :type "Array of Actor Object Reference"))
  (return))

(fn `UserConstructionScript`
  (set `CharacterMovementComponent.MaxWalkSpeed` (`self.WalkingSpeed`) (`self.CharacterMovement`)))