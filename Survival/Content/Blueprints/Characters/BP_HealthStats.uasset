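; BP_HealthStats runs survival stats for health, hunger, thirst and stamina, firing calls when they deplete.
; Each Tick drains hunger and thirst, damages health when either is empty, and moves stamina toward empty or full at a constant rate.
; Health auto-regeneration starts below a low threshold and stops at an upper one or when needs run out.
; Thirst depletion reuses the hunger-end call, and its reset checks Hunger instead of Thirst.
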(event `self.ReceiveTick`
  (params (DeltaSeconds :type "Float (single-precision)"))
  (`|ExecutionSequence`
    (:`then_0`
      (`self.CalculateHunger`)
      (`self.Calculate Thirst`)
      (`self.HungerThirstDamage`)
      (`self.UseStamina` (`self.UsingStamina`) 40.0)
      (`self.HealthRegeneration`))))

(fn `Calculate Thirst`
  (`self.ChangeThirst` (* (`self.ThirstSpeed`) (`GameplayStatics.GetWorldDeltaSeconds`) -1.0)))

(fn `CalculateHunger`
  (`self.ChangeHunger` (* (`self.HungerSpeed`) (`GameplayStatics.GetWorldDeltaSeconds`) -1.0)))

(fn `ChangeHealth`
  (params (Value :type "Float (double-precision)"))
  (bind _output_get (set `self.Health` (`KismetMathLibrary.FMax` (`KismetMathLibrary.FMin` (+ Value (`self.Health`)) (`self.HealthMax`)))))
  (if (and (<= _output_get 0.0) (not (`self.HealthEnded`)))
    (set `self.HealthEnded` true)
    (`self.HealthEnd`)
    (else
      (set `self.HealthEnded` false))))

(fn `ChangeHunger`
  (params (Hunger :type "Float (double-precision)"))
  (bind _output_get (set `self.Hunger` (`KismetMathLibrary.FClamp` (+ Hunger (`self.Hunger`)) 0.0 (`self.HungerMax`))))
  (if (and (<= _output_get 0.0) (not (`self.HungerEnded`)))
    (set `self.HungerEnded` true)
    (`self.HungerEnd`)
    (elif (and (`self.HungerEnded`) (> (`self.Hunger`) 0.0))
      (set `self.HungerEnded` false))))

(fn `ChangeThirst`
  (params (Value :type "Float (double-precision)"))
  (bind _output_get (set `self.Thirst` (`KismetMathLibrary.FClamp` (+ Value (`self.Thirst`)) 0.0 (`self.ThirstMax`))))
  (if (and (<= _output_get 0.0) (not (`self.ThirstEnded`)))
    (set `self.ThirstEnded` true)
    (`self.HungerEnd`)
    (elif (and (`self.ThirstEnded`) (> (`self.Hunger`) 0.0))
      (set `self.ThirstEnded` false))))

(fn `DisplayStats`
  (`|ExecutionSequence`
    (:`then_0`
      (`self.printString` "Health: " (`self.Health`) (struct :`G` 0.442708 :`B` 0.042714 :`A` 1.0)))
    (:`then_1`
      (`self.printString` "Hunger: " (`self.Hunger`) (struct :`R` 0.697917 :`G` 0.499814 :`A` 1.0)))
    (:`then_2`
      (`self.printString` "Thirst: " (`self.Thirst`) (struct :`G` 0.140156 :`B` 0.666667 :`A` 1.0)))
    (:`then_3`
      (`self.printString` "Stamina: " (`self.Stamina`) (struct :`R` 0.087337 :`G` 0.28125 :`B` 0.267248 :`A` 1.0)))))

(fn `HealthRegeneration`
  (`|ExecutionSequence`
    (:`then_0`
      (if (`self.AllowAutoRegeneration`)
        (if (and (< (`self.Health`) (`self.LowLevelRegeneration`)) (not (`self.IsLackOfNeeds`)))
          (set `self.AutoRegeneration` true)
          (elif (or (>= (`self.Health`) (`self.MaxRegenHealth`)) (`self.IsLackOfNeeds`))
            (set `self.AutoRegeneration` false)))))
    (:`then_1`
      (if (or (`self.CanReg`) (`self.AutoRegeneration`))
        (`self.ChangeHealth` (* (`self.RegenerationSpeed`) (`GameplayStatics.GetWorldDeltaSeconds`)))))))

(fn `HungerThirstDamage`
  (if (`self.IsLackOfNeeds`)
    (`self.ChangeHealth` (* (`self.HungerThirtDamageValue`) (`GameplayStatics.GetWorldDeltaSeconds`) -1.0))))

(fn `IsLackOfNeeds`
  (returns (lack :type Boolean))
  (return (or (`self.HungerEnded`) (`self.ThirstEnded`))))

(fn `printString`
  (params (Text :type String) (Value :type "Float (double-precision)") (TextColor :type "LinearColor Structure"))
  (`KismetSystemLibrary.PrintString` (`KismetStringLibrary.Concat_StrStr` Text (`KismetStringLibrary.Conv_DoubleToString` Value)) true true TextColor 0.0))

(fn `UseStamina`
  (params (Use :type Boolean) (UseSpeed :type "Float (double-precision)"))
  (bind _output_get (set `self.UsingStamina` Use))
  (if _output_get
    (set `self.StaminaSpeed` UseSpeed)
    (else
      (set `self.StaminaEnded` false)))
  (bind _output_get_2 (set `self.Stamina` (`KismetMathLibrary.FInterpTo_Constant` (`self.Stamina`) (`KismetMathLibrary.SelectFloat` 0.0 100.0 _output_get) (`GameplayStatics.GetWorldDeltaSeconds`) (`self.StaminaSpeed`))))
  (if (<= _output_get_2 0.0)
    (`self.StaminaEnd`)))