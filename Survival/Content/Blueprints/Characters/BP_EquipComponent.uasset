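; Equipment component for survival characters, player or NPC, that tracks items in head, torso, legs, feet and weapon slots and broadcasts equip changes.
; Equipping attaches hats and weapons to sockets, while clothes follow the body skeleton through master pose.
; For players, torso and weapon use the first-person or body mesh depending on the active camera.
; View switches re-attach items and hide head, leg and foot gear in first person.
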(event `self.ReceiveBeginPlay`
  (bind _assurvival_character (cast `/Game/Blueprints/Characters/SurvivalCharacter` (`self.GetOwner`)))
  (bind _output_get (set `self.SurvivalCharacter` _assurvival_character))
  (bind _assurvival_character_player (cast `/Game/Blueprints/Characters/SurvivalCharacterPlayer` _output_get))
  (add `/Game/Blueprints/Characters/SurvivalCharacterPlayer.OnViewSwitched-SurvivalCharacterPlayer` _assurvival_character_player (delegate `OnViewSwitched-SurvivalCharacterPlayer`)))

(event `OnViewSwitched-SurvivalCharacterPlayer`
  (params (FirstCameraActive :type Boolean))
  (`self.ToggleMeshesVisibilityByCameras` FirstCameraActive))

(fn `AttachClothes`
  (params (ClothesItem :type "/Game/Blueprints/Storage/Items/Equipables/Clothes/ClothesItem Object Reference"))
  (locals (L_ClothesItem :type "/Game/Blueprints/Storage/Items/Equipables/Clothes/ClothesItem Object Reference") (L_SkeletonMeshToAttach :type "SkeletalMeshComponent Object Reference"))
  (`/Engine/EditorBlueprintResources/StandardMacros.IsValid` ClothesItem
    (:`Is Valid`
      (bind _output_get (set `local.L_ClothesItem` ClothesItem))
      (bind _output_get_2 (set `local.L_SkeletonMeshToAttach` (`self.MeshToAttach` _output_get)))
      (`Actor.K2_AttachToComponent` (`local.L_ClothesItem`) _output_get_2 "None" "SnapToTarget" "SnapToTarget" "SnapToTarget" true)
      (`SkinnedMeshComponent.SetLeaderPoseComponent` (`/Game/Blueprints/Storage/Items/Equipables/Clothes/ClothesItem.Clothes` (`local.L_ClothesItem`)) (`local.L_SkeletonMeshToAttach`) false))))

(fn `AttachHat`
  (params (Hat :type "/Game/Blueprints/Storage/Items/Equipables/Clothes/Hats/BP_Hat Object Reference"))
  (`Actor.K2_AttachToComponent` Hat (`self.MeshToAttach` Hat) "Skt_Head" "SnapToTarget" "SnapToTarget" "SnapToTarget" true))

(fn `AttachWeapon`
  (params (Attach :type Boolean))
  (`/Engine/EditorBlueprintResources/StandardMacros.IsValid` (`self.Weapon`)
    (:`Is Valid`
      (if Attach
        (`Actor.K2_AttachToComponent` (`self.Weapon`) (`self.MeshToAttach` (`self.Weapon`)) "Skt_Weapon" "SnapToTarget" "SnapToTarget" "SnapToTarget" true)
        (else
          (`Actor.K2_DetachFromActor` (`self.Weapon`) "KeepRelative" "KeepRelative" "KeepRelative"))))))

(fn `EquipClothes`
  (params (Item :type "/Game/Blueprints/Storage/Items/BP_StorageItem Object Reference"))
  (locals (L_ClothesItem :type "/Game/Blueprints/Storage/Items/Equipables/Clothes/ClothesItem Object Reference"))
  (bind _asclothes_item (cast `/Game/Blueprints/Storage/Items/Equipables/Clothes/ClothesItem` Item))
  (bind _output_get (set `local.L_ClothesItem` _asclothes_item))
  (switch `/Game/Blueprints/Storage/Items/Equipables/E_EquipPart` (`/Game/Blueprints/Storage/Items/Equipables/EquipableItem.EquipPart` _output_get)
    (:`NewEnumerator1`
      (set `self.Torso` (`local.L_ClothesItem`)))
    (:`NewEnumerator2`
      (set `self.Legs` (`local.L_ClothesItem`)))
    (:`NewEnumerator3`
      (set `self.Foots` (`local.L_ClothesItem`))))
  (`self.AttachClothes` (`local.L_ClothesItem`)))

(fn `EquipHat`
  (params (Item :type "/Game/Blueprints/Storage/Items/BP_StorageItem Object Reference"))
  (locals (L_Item :type "/Game/Blueprints/Storage/Items/BP_StorageItem Object Reference"))
  (bind _output_get (set `local.L_Item` Item))
  (bind _asbp_hat (cast `/Game/Blueprints/Storage/Items/Equipables/Clothes/Hats/BP_Hat` _output_get))
  (set `self.Head` _asbp_hat)
  (bind _assurvival_character_player (cast `/Game/Blueprints/Characters/SurvivalCharacterPlayer` (`self.SurvivalCharacter`))
    (:`then`
      (if (`/Game/Blueprints/Characters/SurvivalCharacterPlayer.FirstCameraActive` _assurvival_character_player)
        (`Actor.SetActorHiddenInGame` (`self.Head`) true)
        (else
          (`self.AttachHat` (`self.Head`) :!label _label))))
    (:`CastFailed`
      (goto _label))))

(fn `EquipItem`
  (params (Item :type "/Game/Blueprints/Storage/Items/Equipables/EquipableItem Object Reference") (Part :type "/Game/Blueprints/Storage/Items/Equipables/E_EquipPart Enum" :default "NewEnumerator0"))
  (returns (Equipped :type Boolean))
  (locals (L_Item :type "/Game/Blueprints/Storage/Items/Equipables/EquipableItem Object Reference") (L_Part :type "/Game/Blueprints/Storage/Items/Equipables/E_EquipPart Enum" :default "NewEnumerator0"))
  (set `local.L_Item` Item)
  (set `local.L_Part` Part)
  (`/Game/Blueprints/Storage/Items/Equipables/EquipableItem.UnEquipItem` (`local.L_Item`))
  (switch `/Game/Blueprints/Storage/Items/Equipables/E_EquipPart` (`local.L_Part`)
    (:`NewEnumerator0`
      (`self.EquipHat` (`local.L_Item`)))
    (:`NewEnumerator1`
      (`self.EquipClothes` (`local.L_Item`) :!label _label))
    (:`NewEnumerator2`
      (goto _label))
    (:`NewEnumerator3`
      (goto _label))
    (:`NewEnumerator4`
      (`self.EquipWeapon` (`local.L_Item`))))
  (`self.OnItemEquiped-BP_EquipComponent` (`local.L_Item`))
  (return true))

(fn `EquipWeapon`
  (params (Item :type "/Game/Blueprints/Storage/Items/Equipables/EquipableItem Object Reference"))
  (bind _asweapon (cast `/Game/Blueprints/Storage/Items/Equipables/Weapons/Weapon` Item))
  (set `self.Weapon` _asweapon)
  (`self.AttachWeapon` true)
  (`self.OnWeaponEquiped-BP_EquipComponent` (`self.Weapon`)))

(fn `MeshToAttach`
  (params (Item :type "/Game/Blueprints/Storage/Items/Equipables/EquipableItem Object Reference"))
  (returns (SkeletonMesh :type "SkeletalMeshComponent Object Reference"))
  (locals (NewLocalVar_0 :type "/Game/Blueprints/Storage/Items/Equipables/E_EquipPart Enum" :default "NewEnumerator0") (L_Item :type "/Game/Blueprints/Storage/Items/Equipables/EquipableItem Object Reference"))
  (bind _mesh (`Character.Mesh` (`self.SurvivalCharacter`)))
  (bind _mesh_2 (`Character.Mesh` (`self.SurvivalCharacter`)))
  (set `local.L_Item` Item)
  (bind _assurvival_character_player (cast `/Game/Blueprints/Characters/SurvivalCharacterPlayer` (`self.SurvivalCharacter`))
    (:`then`
      (bind _returnvalue (select `bool` (`/Game/Blueprints/Characters/SurvivalCharacterPlayer.FirstCameraActive` _assurvival_character_player) :`false` (`Character.Mesh` _assurvival_character_player) :`true` (`/Game/Blueprints/Characters/SurvivalCharacterPlayer.FirstPersonMesh` _assurvival_character_player)))
      (return (select `/Game/Blueprints/Storage/Items/Equipables/E_EquipPart` (`/Game/Blueprints/Storage/Items/Equipables/EquipableItem.EquipPart` (`local.L_Item`)) :`NewEnumerator0` _mesh :`NewEnumerator1` _returnvalue :`NewEnumerator2` _mesh :`NewEnumerator3` _mesh :`NewEnumerator4` _returnvalue)))
    (:`CastFailed`
      (return (select `/Game/Blueprints/Storage/Items/Equipables/E_EquipPart` (`/Game/Blueprints/Storage/Items/Equipables/EquipableItem.EquipPart` (`local.L_Item`)) :`NewEnumerator0` _mesh_2 :`NewEnumerator1` _mesh_2 :`NewEnumerator2` _mesh_2 :`NewEnumerator3` _mesh_2 :`NewEnumerator4` _mesh_2)))))

(fn `PartEquipped`
  (params (Part :type "/Game/Blueprints/Storage/Items/Equipables/E_EquipPart Enum" :default "NewEnumerator0"))
  (returns (Equipped :type Boolean) (Item :type "/Game/Blueprints/Storage/Items/Equipables/EquipableItem Object Reference"))
  (bind _returnvalue (select `/Game/Blueprints/Storage/Items/Equipables/E_EquipPart` Part :`NewEnumerator0` (`self.Head`) :`NewEnumerator1` (`self.Torso`) :`NewEnumerator2` (`self.Legs`) :`NewEnumerator3` (`self.Foots`) :`NewEnumerator4` (`self.Weapon`) :!type "/Game/Blueprints/Storage/Items/Equipables/EquipableItem Object Reference"))
  (return (`KismetSystemLibrary.IsValid` _returnvalue) _returnvalue))

(fn `ToggleMeshesVisibilityByCameras`
  (params (InputPin :type Boolean))
  (bind _head (`self.Head`))
  (bind _legs (`self.Legs`))
  (bind _foots (`self.Foots`))
  (`self.AttachClothes` (`self.Torso`))
  (`self.AttachWeapon` true)
  (`/Engine/EditorBlueprintResources/StandardMacros.IsValid` _head
    (:`Is Valid`
      (`Actor.SetActorHiddenInGame` _head InputPin)
      (`self.AttachHat` _head))
    (:`Is Not Valid`
      _))
  (`/Engine/EditorBlueprintResources/StandardMacros.IsValid` _legs
    (:`Is Valid`
      (`Actor.SetActorHiddenInGame` _legs InputPin)
      (`self.AttachClothes` _legs))
    (:`Is Not Valid`
      _))
  (`/Engine/EditorBlueprintResources/StandardMacros.IsValid` _foots
    (:`Is Valid`
      (`Actor.SetActorHiddenInGame` _foots InputPin))))

(fn `Un Equip Item`
  (params (Part :type "/Game/Blueprints/Storage/Items/Equipables/E_EquipPart Enum" :default "NewEnumerator0"))
  (returns (Unequipped :type Boolean))
  (locals (L_UnequipedItem :type "/Game/Blueprints/Storage/Items/Equipables/EquipableItem Object Reference"))
  (bind (_equipped _item) (`self.PartEquipped` Part))
  (if _equipped
    (set `local.L_UnequipedItem` _item)
    (switch `/Game/Blueprints/Storage/Items/Equipables/E_EquipPart` Part
      (:`NewEnumerator0`
        (set `self.Head` null))
      (:`NewEnumerator1`
        (set `self.Torso` null))
      (:`NewEnumerator2`
        (set `self.Legs` null))
      (:`NewEnumerator3`
        (set `self.Foots` null))
      (:`NewEnumerator4`
        (set `self.Weapon` null)))
    (`self.OnItemUnequiped-BP_EquipComponent` (`local.L_UnequipedItem`))
    (return true)
    (else
      (return false))))