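; Survival game instance that manages level loading screens, saving and loading, and creates the hero targets info object on init.
; All slots share one save object, with each save inserted first in its array.
; Saves capture player stats, components, view, settings and nearby actor/component transforms via a huge sphere trace.
; Loading applies the first name-matching slot, caches world transforms and broadcasts completion; the older save/load paths and transform-restore logic are disconnected.
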(event `self.ReceiveInit`
  (bind _outactors (`GameplayStatics.GetAllActorsOfClass` "/Game/Blueprints/Other/DayHightCircle/BP_DayHightCircle.BP_DayHightCircle_C"))
  (set `self.DayHightCircle` (`|GetArrayItem` _outactors))
  (`self.InitTargetsInfo`))

(event `LoadLevel`
  (params (LevelName :type Name))
  (set `self.LevelToOpen` LevelName)
  (`self.ShowLoadWidget`))

(event `CloseLoadScreen`
  (`/Engine/EditorBlueprintResources/StandardMacros.IsValid` (`self.W_LoadScreen`)
    (:`Is Valid`
      (`Widget.RemoveFromParent` (`self.W_LoadScreen`))
      (set `self.W_LoadScreen` null))))

(event `LoadGame`
  (params (SlotName :type Text))
  (bind _bp_healthstats (`/Game/Blueprints/Characters/SurvivalCharacter.BP_HealthStats` (`self.SurvivalCharacter`)))
  (bind _assurvival_character_player (cast `/Game/Blueprints/Characters/SurvivalCharacterPlayer` (`GameplayStatics.GetPlayerCharacter` 0)))
  (set `self.SurvivalCharacter` _assurvival_character_player)
  (bind _assurvival_player_controller (cast `/Game/Blueprints/GameMode/SurvivalPlayerController` (`GameplayStatics.GetPlayerController` 0)))
  (set `self.SurvivalPlayerController` _assurvival_player_controller)
  (set `self.SlotName` SlotName)
  ;[1 1 1] checking save game slot
  (bind _returnvalue (`GameplayStatics.DoesSaveGameExist` (`/Game/Blueprints/Lib.GetOverallSaveGameObjName`)))
  (if _returnvalue
    (bind _returnvalue_2 (`GameplayStatics.LoadGameFromSlot` (`/Game/Blueprints/Lib.GetOverallSaveGameObjName`)))
    (bind _assave_game_slot (cast `/Game/Save/SaveGameSlot` _returnvalue_2))
    (set `self.LoadGameRef` _assave_game_slot)
    (for _array_element (`/Game/Save/SaveGameSlot.SaveGameSlotsArray` (`self.LoadGameRef`))
      (bind (_slotname _savedate _allsaveparamsstructure) (break `/Game/Save/SaveStructures/ST_SaveSlotStructure` _array_element))
      (if (`KismetTextLibrary.EqualEqual_TextText` _slotname (`self.SlotName`))
        (bind (_charactertransform _controlcamerarotation _storagecomponent _equipcomponent _healthcomponent _dayhightcircle _soundvolume _allcomponentsaroundarray _allcomponentstransforms _allactorsaroundarray _allactorsaroundtransform _firstperson _herotargetsinfocomponent _thirst _hunger _stamina _health _startgamecutsceneplayed) (break `/Game/Save/SaveStructures/ST_AllSaveParams` _allsaveparamsstructure))
        (set `/Game/Blueprints/Characters/BP_HealthStats.Health` _health _bp_healthstats)
        (set `/Game/Blueprints/Characters/BP_HealthStats.Thirst` _thirst _bp_healthstats)
        (set `/Game/Blueprints/Characters/BP_HealthStats.Hunger` _hunger _bp_healthstats)
        (set `/Game/Blueprints/Characters/BP_HealthStats.Stamina` _stamina _bp_healthstats)
        (`Actor.K2_SetActorTransform` (`self.SurvivalCharacter`) _charactertransform false false)
        (`Controller.SetControlRotation` (`GameplayStatics.GetPlayerController` 0) _controlcamerarotation)
        (set `/Game/Blueprints/Characters/SurvivalCharacter.BP_StorageComponent` _storagecomponent (`self.SurvivalCharacter`))
        (set `/Game/Blueprints/Characters/SurvivalCharacter.BP_EquipedComponent` _equipcomponent (`self.SurvivalCharacter`))
        (set `/Game/Blueprints/Characters/SurvivalCharacter.BP_HealthStats` _healthcomponent (`self.SurvivalCharacter`))
        (set `self.DayHightCircle` _dayhightcircle)
        (bind _output_get (set `self.SoundVolume` _soundvolume))
        (`GameplayStatics.SetSoundMixClassOverride` "/Game/Assets/Music/OverallGameSounds/SCM_AllGameSounds.SCM_AllGameSounds" "/Game/Assets/Music/OverallGameSounds/SC_AllGameSounds.SC_AllGameSounds" _output_get)
        (set `self.AllComponentsAroundArray` _allcomponentsaroundarray)
        (set `self.AllComponentsAroundTransforms` _allcomponentstransforms)
        (set `self.AllActorsAroundArray` _allactorsaroundarray)
        (set `self.AllActorsAroundTransform` _allactorsaroundtransform)
        (set `/Game/Blueprints/GameMode/SurvivalPlayerController.FirstPerson` _firstperson (`self.SurvivalPlayerController`))
        (set `self.StartGameCutScenePlayed` _startgamecutsceneplayed)
        (`self.OnAllParamsLoaded-SurvivalGameInstance`)
        (break)))))

(event `SaveGameToSlot`
  (params (SaveGameSlot :type "/Game/Save/SaveStructures/ST_SaveSlotStructure Structure"))
  (bind (_slotname _savedate) (break `/Game/Save/SaveStructures/ST_SaveSlotStructure` SaveGameSlot))
  (bind (_allcomponentsaroundarray _allcomponentsaroundtransforms _allactorsaroundarray _allactorsaroundtransform) (`self.SaveTransformAllActors`))
  (bind _survivalcharacter (`self.SurvivalCharacter`))
  (bind _survivalcharacter_2 (`self.SurvivalCharacter`))
  (bind _bp_healthstats (`/Game/Blueprints/Characters/SurvivalCharacter.BP_HealthStats` (`self.SurvivalCharacter`)))
  (bind _st_allsaveparams (make `/Game/Save/SaveStructures/ST_AllSaveParams` (`Actor.GetTransform` _survivalcharacter_2) (`Pawn.GetControlRotation` _survivalcharacter_2) (`/Game/Blueprints/Characters/SurvivalCharacter.BP_StorageComponent` _survivalcharacter) (`/Game/Blueprints/Characters/SurvivalCharacter.BP_EquipedComponent` _survivalcharacter) (`/Game/Blueprints/Characters/SurvivalCharacter.BP_HealthStats` _survivalcharacter) (`self.DayHightCircle`) (`self.SoundVolume`) _allcomponentsaroundarray _allcomponentsaroundtransforms _allactorsaroundarray _allactorsaroundtransform (`/Game/Blueprints/GameMode/SurvivalPlayerController.FirstPerson` (cast `/Game/Blueprints/GameMode/SurvivalPlayerController` (`GameplayStatics.GetPlayerController` 0) :!pure true)) null (`/Game/Blueprints/Characters/BP_HealthStats.Thirst` _bp_healthstats) (`/Game/Blueprints/Characters/BP_HealthStats.Hunger` _bp_healthstats) (`/Game/Blueprints/Characters/BP_HealthStats.Stamina` _bp_healthstats) (`/Game/Blueprints/Characters/BP_HealthStats.Health` _bp_healthstats) (`self.StartGameCutScenePlayed`)))
  (bind _assurvival_character_player (cast `/Game/Blueprints/Characters/SurvivalCharacterPlayer` (`GameplayStatics.GetPlayerCharacter` 0)))
  (set `self.SurvivalCharacter` _assurvival_character_player)
  (set `self.SlotName` _slotname)
  (set `self.SaveDate` _savedate)
  (bind _returnvalue (`GameplayStatics.DoesSaveGameExist` (`/Game/Blueprints/Lib.GetOverallSaveGameObjName`)))
  (if _returnvalue
    (bind _returnvalue_2 (`GameplayStatics.LoadGameFromSlot` (`/Game/Blueprints/Lib.GetOverallSaveGameObjName`)))
    (bind _assave_game_slot (cast `/Game/Save/SaveGameSlot` _returnvalue_2))
    (`KismetArrayLibrary.Array_Insert` (`/Game/Save/SaveGameSlot.SaveGameSlotsArray` _assave_game_slot) (make `/Game/Save/SaveStructures/ST_SaveSlotStructure` (`self.SlotName`) (`self.SaveDate`) _st_allsaveparams))
    (`GameplayStatics.SaveGameToSlot` _assave_game_slot (`/Game/Blueprints/Lib.GetOverallSaveGameObjName`))
    (else
      (bind _returnvalue_3 (`GameplayStatics.CreateSaveGameObject` "/Game/Save/SaveGameSlot.SaveGameSlot_C"))
      (`KismetArrayLibrary.Array_Insert` (`/Game/Save/SaveGameSlot.SaveGameSlotsArray` _returnvalue_3) (make `/Game/Save/SaveStructures/ST_SaveSlotStructure` (`self.SlotName`) (`self.SaveDate`) _st_allsaveparams))
      (`GameplayStatics.SaveGameToSlot` _returnvalue_3 (`/Game/Blueprints/Lib.GetOverallSaveGameObjName`)))))

(fn `InitTargetsInfo`
  (bind _returnvalue (`|GenericCreateObject` (`self.HeroTargetsInfoClass`) self))
  (set `self.HeroTargetsInfo` _returnvalue))

(fn `LoadHealthsStats`)

(fn `LoadTransformAllActors`)

(fn `SaveHealthsStats`
  (set `/Game/Save/Savegame_BP.HealthComponent` (`/Game/Blueprints/Characters/SurvivalCharacter.BP_HealthStats` (`self.SurvivalCharacter`)) (`self.SaveGameRef`))
  (set `/Game/Save/Savegame_BP.Health` (`/Game/Blueprints/Characters/BP_HealthStats.Health` (`/Game/Blueprints/Characters/SurvivalCharacter.BP_HealthStats` (`self.SurvivalCharacter`))) (`self.SaveGameRef`))
  (set `/Game/Save/Savegame_BP.Hunger` (`/Game/Blueprints/Characters/BP_HealthStats.Hunger` (`/Game/Blueprints/Characters/SurvivalCharacter.BP_HealthStats` (`self.SurvivalCharacter`))) (`self.SaveGameRef`))
  (set `/Game/Save/Savegame_BP.Stamina` (`/Game/Blueprints/Characters/BP_HealthStats.Stamina` (`/Game/Blueprints/Characters/SurvivalCharacter.BP_HealthStats` (`self.SurvivalCharacter`))) (`self.SaveGameRef`))
  (set `/Game/Save/Savegame_BP.Thirst` (`/Game/Blueprints/Characters/BP_HealthStats.Thirst` (`/Game/Blueprints/Characters/SurvivalCharacter.BP_HealthStats` (`self.SurvivalCharacter`))) (`self.SaveGameRef`)))

(fn `SaveTransformAllActors`
  (returns (AllComponentsAroundArray :type "Array of PrimitiveComponent Object Reference") (AllComponentsAroundTransforms :type "Array of Transform Structure") (AllActorsAroundArray :type "Array of Actor Object Reference") (AllActorsAroundTransform :type "Array of Transform Structure"))
  (bind _survivalcharacter (`self.SurvivalCharacter`)
    (:`then`
      (bind _returnvalue (`Actor.K2_GetActorLocation` _survivalcharacter))
      (bind (_outhits _returnvalue_2) (`KismetSystemLibrary.SphereTraceMultiForObjects` :`Start` _returnvalue :`End` _returnvalue :`Radius` 1000000.0 :`ObjectTypes` (`|MakeArray` "ObjectTypeQuery1" "ObjectTypeQuery2" "ObjectTypeQuery3" "ObjectTypeQuery4" "ObjectTypeQuery5" "ObjectTypeQuery6" :!type "EObjectTypeQuery Enum") :`DrawTime` 0.0))
      (if _returnvalue_2
        (`KismetArrayLibrary.Array_Clear` (`self.AllComponentsAroundArray`))
        (`KismetArrayLibrary.Array_Clear` (`self.AllComponentsAroundTransforms`))
        (`KismetArrayLibrary.Array_Clear` (`self.AllActorsAroundArray`))
        (`KismetArrayLibrary.Array_Clear` (`self.AllActorsAroundTransform`))
        (for _array_element _outhits
          (`KismetArrayLibrary.Array_Add` (`self.AllComponentsAroundArray`) (`.HitComponent` (`GameplayStatics.BreakHitResult` _array_element)))
          (`KismetArrayLibrary.Array_Add` (`self.AllComponentsAroundTransforms`) (`SceneComponent.K2_GetComponentToWorld` (`.HitComponent` (`GameplayStatics.BreakHitResult` _array_element))))
          (`KismetArrayLibrary.Array_Add` (`self.AllActorsAroundArray`) (`.HitActor` (`GameplayStatics.BreakHitResult` _array_element)))
          (`KismetArrayLibrary.Array_Add` (`self.AllActorsAroundTransform`) (`Actor.GetTransform` (`.HitActor` (`GameplayStatics.BreakHitResult` _array_element)))))
        (return (`self.AllComponentsAroundArray`) (`self.AllComponentsAroundTransforms`) (`self.AllActorsAroundArray`) (`self.AllActorsAroundTransform`))))
    (:`else`)))

(fn `ShowLoadWidget`
  (bind _returnvalue (`|CreateWidget` "/Game/UI/LoadScreen/W_LoadScreen.W_LoadScreen_C" (`GameplayStatics.GetPlayerController` 0) (`self.LevelToOpen`)))
  (bind _output_get (set `self.W_LoadScreen` _returnvalue))
  (`UserWidget.AddToViewport` _output_get 0)
  (`/Game/UI/LoadScreen/W_LoadScreen.FadeInOut` (`self.W_LoadScreen`)))