(event `self.ReceiveBeginPlay`
  (`|ExecutionSequence`
    (:`then_0`
      (bind _returnvalue (`|CreateWidget` "/Game/UI/MainHUD/BP_HUD.BP_HUD_C" self))
      (bind _output_get (set `self.W_HUD` _returnvalue))
      (`UserWidget.AddToViewport` _output_get 0))
    (:`then_1`
      (bind _returnvalue_2 (`|CreateWidget` "/Game/UI/Inventary/BW_Inventory.BW_Inventory_C" self))
      (set `self.W_Inventory` _returnvalue_2))))

(event `Key|I`
  (params (Key :type "Key Structure"))
  (:`Pressed`
    (`self.ToggleInventory`)))

(event `Key|BackSpace`
  (params (Key :type "Key Structure"))
  (:`Pressed`
    (`|ExecutionSequence` :!label _label
      (:`then_0`
        (`/Engine/EditorBlueprintResources/StandardMacros.IsValid` (`self.W_ExchangeWidget`)
          (:`Is Valid`
            (`self.ExchangeWidget` null true)
            (`self.OnBoxClosed` (`self.ProcessPlayBoxCoverOpeningAnim`)))))
      (:`then_1`
        (`/Engine/EditorBlueprintResources/StandardMacros.IsValid` (`self.W_CraftWidget`)
          (:`Is Valid`
            (`self.CraftWidget` false)))))))

(event `Key|Escape`
  (params (Key :type "Key Structure"))
  (:`Pressed`
    (goto _label)))

(fn `ControlUI`
  (params (InventoryWidget :type "UserWidget Object Reference") (Activate :type Boolean))
  (locals (L_InventoryWidget :type "UserWidget Object Reference"))
  (set `local.L_InventoryWidget` InventoryWidget)
  (if Activate
    (set `self.bShowMouseCursor` true)
    (`/Engine/EditorBlueprintResources/StandardMacros.IsValid` (`local.L_InventoryWidget`)
      (:`Is Valid`
        (`WidgetBlueprintLibrary.SetInputMode_GameAndUIEx` self (`local.L_InventoryWidget`) "DoNotLock" false)
        (`self.DisableInput` (`self.K2_GetPawn`) self))
      (:`Is Not Valid`
        (`KismetSystemLibrary.PrintString` "Inventory Widget input param is not assigned")))
    (else
      (set `self.bShowMouseCursor` false)
      (`self.EnableInput` (`self.K2_GetPawn`) self)
      (`WidgetBlueprintLibrary.SetInputMode_GameOnly` self))))

(fn `CraftWidget`
  (params (Show :type Boolean))
  (returns (CraftWidget :type "/Game/UI/Craft/WB_CraftWindow Object Reference"))
  (if Show
    (bind _returnvalue (`|CreateWidget` "/Game/UI/Craft/WB_CraftWindow.WB_CraftWindow_C" self))
    (bind _output_get (set `self.W_CraftWidget` _returnvalue))
    (`UserWidget.AddToViewport` _output_get 0)
    (`self.ControlUI` (`self.W_CraftWidget`) true)
    (return (`self.W_CraftWidget`))
    (else
      (`Widget.RemoveFromParent` (`self.W_CraftWidget`))
      (set `self.W_CraftWidget` null)
      (`self.ControlUI` null))))

(fn `ExchangeWidget`
  (params (StorageComponent :type "/Game/Blueprints/Storage/BP_StorageComponent Object Reference") (ToRemove :type Boolean))
  (locals (L_StorageComponent :type "/Game/Blueprints/Storage/BP_StorageComponent Object Reference"))
  (set `local.L_StorageComponent` StorageComponent)
  (if (not (`self.ExchangeInventoryShown`))
    (if ToRemove
      (`Widget.RemoveFromParent` (`self.W_ExchangeWidget`) :!label _label)
      (set `self.W_ExchangeWidget` null)
      (`self.ControlUI` (`self.W_ExchangeWidget`))
      (set `self.ExchangeInventoryShown` false)
      (else
        (bind _returnvalue (`|CreateWidget` "/Game/UI/Inventary/BW_ItemExchange.BW_ItemExchange_C" self (`local.L_StorageComponent`)))
        (bind _output_get (set `self.W_ExchangeWidget` _returnvalue))
        (`UserWidget.AddToViewport` _output_get 0)
        (`self.ControlUI` (`self.W_ExchangeWidget`) true)
        (set `self.ExchangeInventoryShown` true)))
    (else
      (goto _label))))

(fn `ProcessPlayBoxCoverOpeningAnim`
  (returns (CurrentInteractedBox :type "/Game/Blueprints/Prefabs/BP_BoxModel Object Reference"))
  (bind _currentinteractedbox (`self.CurrentInteractedBox`))
  (bind _currentinteractedbox_2 (`self.CurrentInteractedBox`))
  (`/Engine/EditorBlueprintResources/StandardMacros.IsValid` _currentinteractedbox_2
    (:`Is Valid`
      (if (not (`/Game/Blueprints/Prefabs/BP_BoxModel.Closed` _currentinteractedbox_2))
        (set `/Game/Blueprints/Prefabs/BP_BoxModel.Closed` true _currentinteractedbox)
        (return _currentinteractedbox)
        (else
          _)))
    (:`Is Not Valid`
      _))
  (return null))

(fn `ToggleInventory`
  (if (not (`self.ExchangeInventoryShown`))
    (if (not (`self.PlayerInventoryShownToggler`))
      ;[1 1 1] Show inventory, block character input
      (`UserWidget.AddToViewport` (`self.W_Inventory`) 0)
      (`/Game/UI/Inventary/BW_Inventory.InvertoryAddedToViewport` (`self.W_Inventory`))
      (set `self.PlayerInventoryShownToggler` true)
      (`self.ControlUI` (`self.W_Inventory`) true)
      (else
        ;[1 1 1] Hide inventory, return inputs
        (`Widget.RemoveFromParent` (`self.W_Inventory`))
        (set `self.PlayerInventoryShownToggler` false)
        (`self.ControlUI` null)))))

(fn `UserConstructionScript`)