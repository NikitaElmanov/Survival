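; Zombie enemy NPC Blueprint that arms itself with a hands weapon at spawn and otherwise relies on its parent class.
; On BeginPlay it runs the parent logic, then spawns BP_Weapon_Zombie_Hands as owner and instigator and stores it as Weapon.
; The weapon has its physics components frozen and is teleported below the world origin before being equipped to the zombie.
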(event `self.ReceiveBeginPlay`
  (`parent.ReceiveBeginPlay`)
  (bind _returnvalue (`|SpawnActorFromClass` "/Game/Blueprints/Storage/Items/Equipables/Weapons/BP_Weapon_Zombie_Hands.BP_Weapon_Zombie_Hands_C" (`KismetMathLibrary.MakeTransform` (0.0 0.0 0.0)) "Undefined" "OverrideRootScale" self 1 self))
  (bind _output_get (set `self.Weapon` _returnvalue))
  (`/Game/Blueprints/Storage/Items/BP_StorageItem.Freeze Physics Components` _output_get true)
  (`self.K2_SetActorLocation` (`self.Weapon`) (0.0 0.0 -1000.0) false true)
  (`self.SetActorHiddenInGame` (`self.Weapon`) false)
  (`/Game/Blueprints/Storage/Items/Equipables/EquipableItem.EquipItem` (`self.Weapon`) self))

(fn `UserConstructionScript`
  (`parent.UserConstructionScript`))