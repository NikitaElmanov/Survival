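; AI controller Blueprint for NPC characters that manages a set of modular control components.
; On possession it caches the NPC pawn, initializes every MainNPCControlComponent and binds to the NPC's alarm and death events and the follow component's destination-reached event.
; Death stops all components, clears the alarm target and destroys the controller.
; The alarm handler only prints a debug string, and the destination-reached handler is empty.
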(event `self.ReceivePossess`
  (params (PossessedPawn :type "Pawn Object Reference"))
  (`self.Init`))

(fn `BindEvents`
  (add `/Game/Blueprints/NPC/NPCCharacter.NPCAlarmed` (`self.NPC`) (`|CreateDelegate` :!event `NPCAlarmed`))
  (add `/Game/Blueprints/Characters/SurvivalCharacter.CharDead` (`self.NPC`) (`|CreateDelegate` :!event `Dead`))
  (add `/Game/Blueprints/NPC/Components/NPCFollowComponent.DestReached` (`self.NPCFollowComponent`) (`|CreateDelegate` :!event `FollowDestReached`)))

(fn `Dead`
  (params (Character :type "/Game/Blueprints/Characters/SurvivalCharacter Object Reference"))
  (`self.StopAllAction`)
  (set `self.AlarmTarget` null)
  (`self.K2_DestroyActor`))

(fn `FollowDestReached`)

(fn `Init`
  (bind _asnpccharacter (cast `/Game/Blueprints/NPC/NPCCharacter` (`self.K2_GetPawn`)))
  (set `self.NPC` _asnpccharacter)
  (for _array_element (`self.K2_GetComponentsByClass` "/Game/Blueprints/NPC/Components/MainNPCControlComponent.MainNPCControlComponent_C")
    (bind _asmain_npccontrol_component (cast `/Game/Blueprints/NPC/Components/MainNPCControlComponent` _array_element))
    (`/Game/Blueprints/NPC/Components/MainNPCControlComponent.Init` _asmain_npccontrol_component))
  (`self.BindEvents`))

(fn `NPCAlarmed`
  (params (Instigator :type "Pawn Object Reference"))
  (`KismetSystemLibrary.PrintString` "NPC alarmed"))

(fn `StopAllAction`
  (returns (Stopped :type Boolean))
  (set `self.AlarmTarget` null)
  (for _array_element (`self.K2_GetComponentsByClass` "/Game/Blueprints/NPC/Components/MainNPCControlComponent.MainNPCControlComponent_C")
    (bind _asmain_npccontrol_component (cast `/Game/Blueprints/NPC/Components/MainNPCControlComponent` _array_element))
    (`/Game/Blueprints/NPC/Components/MainNPCControlComponent.Stop` _asmain_npccontrol_component))
  (return false))

(fn `UserConstructionScript`)