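; Base NPC character for a survival game that reacts to player attacks, fights with its equipped weapon and can be looted once dead.
; Player damage alarms it into sprint speed, fires an alarmed event and alerts nearby NPCs whose class matches its friend list.
; Attack calls drive the weapon in melee or normal mode, and a helper interpolates yaw toward a direction.
; Interacting with the corpse opens a storage exchange widget.
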(event `self.ReceiveAnyDamage`
  (params (Damage :type "Float (single-precision)") (DamageType :type "DamageType Object Reference") (InstigatedBy :type "Controller Object Reference") (DamageCauser :type "Actor Object Reference"))
  (bind _returnvalue (`GameplayStatics.GetPlayerCharacter` 0))
  ;[1 1 1] Alarm by damage
  (`parent.ReceiveAnyDamage` Damage DamageType InstigatedBy DamageCauser)
  (if (== InstigatedBy (`GameplayStatics.GetPlayerController` 0))
    (`self.Alarm` _returnvalue)
    (`self.AlarmFriends` _returnvalue)))

(event `Attack`
  (params (Target :type "Actor Object Reference") (asMelee :type Boolean))
  (bind _weapon (`/Game/Blueprints/Characters/BP_EquipComponent.Weapon` (`self.BP_EquipedComponent`)))
  (set `self.Attacking` true)
  (`/Engine/EditorBlueprintResources/StandardMacros.IsValid` _weapon
    (:`Is Valid`
      (`/Game/Blueprints/Storage/Items/Equipables/Weapons/Weapon.UseWeapon` _weapon true asMelee))))

(event `StopAttack`
  (bind _weapon (`/Game/Blueprints/Characters/BP_EquipComponent.Weapon` (`self.BP_EquipedComponent`)))
  (set `self.Attacking` false)
  (`/Engine/EditorBlueprintResources/StandardMacros.IsValid` _weapon
    (:`Is Valid`
      (`/Game/Blueprints/Storage/Items/Equipables/Weapons/Weapon.UseWeapon` _weapon false false))))

(fn `Alarm`
  (params (Instigator :type "Pawn Object Reference"))
  (locals (L_Instiator :type "Pawn Object Reference"))
  (if (and (not (`self.Alarmed`)) (not (`self.Dead`)))
    (set `local.L_Instiator` Instigator)
    (set `self.Alarmed` true)
    (set `CharacterMovementComponent.MaxWalkSpeed` (`self.SprintingSpeed`) (`self.CharacterMovement`))
    (set `self.IsSprinting` true)
    (`self.NPCAlarmed-NPCCharacter` (`local.L_Instiator`))))

(fn `AlarmFriends`
  (params (Instigator :type "Pawn Object Reference"))
  (locals (L_ArrayElem :type "/Game/Blueprints/NPC/NPCCharacter Object Reference") (L_Instigator :type "Pawn Object Reference"))
  (set `local.L_Instigator` Instigator)
  (bind _outactors (`GameplayStatics.GetAllActorsOfClass` "NPCCharacter_C"))
  (for _array_element _outactors
    (bind _output_get (set `local.L_ArrayElem` _array_element))
    (if (!= _output_get self)
      (if (<= (`KismetMathLibrary.VSize` (- (`self.K2_GetActorLocation` (`local.L_ArrayElem`)) (`self.K2_GetActorLocation`))) (`self.AlarmFriendsRadius`))
        (if (`self.IsFriend` (`local.L_ArrayElem`))
          (`self.Alarm` (`local.L_ArrayElem`) (`local.L_Instigator`)))))))

(fn `Interact`
  (params (Character :type "/Game/Blueprints/Characters/SurvivalCharacter Object Reference"))
  (returns (Successfull :type Boolean) (Message :type String))
  (if (`self.Dead`)
    (bind _assurvival_player_controller (cast `/Game/Blueprints/GameMode/SurvivalPlayerController` (`self.GetController` Character))
      (:`then`
        (`/Game/Blueprints/GameMode/SurvivalPlayerController.ExchangeWidget` _assurvival_player_controller (`self.BP_StorageComponent`) false)
        (return true ""))
      (:`CastFailed`
        (return false "cast failed")))
    (else
      (return false "npc isn't dead"))))

(fn `IsFriend`
  (params (Pawn :type "Object Object Reference"))
  (returns (Out :type Boolean))
  (bind _returnvalue (`GameplayStatics.GetObjectClass` Pawn))
  (for _array_element (`self.FriendList`)
    (if (or (== _array_element _returnvalue) (`KismetMathLibrary.ClassIsChildOf` _returnvalue _array_element))
      (return true)))
  (return false))

(fn `RotateTowardsDirection`
  (params (DeltaTime :type "Float (double-precision)") (InterpSpeed :type "Float (double-precision)") (Direction :type "Vector Structure") (RotatedThreshold :type "Float (double-precision)"))
  (returns (Rotated :type Boolean))
  (bind (_returnvalue_roll _returnvalue_pitch _returnvalue_yaw) (`KismetMathLibrary.BreakRotator` (`self.K2_GetActorRotation`)))
  (bind _returnvalue (`self.GetController`))
  (bind (_returnvalue_roll_2 _returnvalue_pitch_2 _returnvalue_yaw_2) (`KismetMathLibrary.BreakRotator` (`self.K2_GetActorRotation`)))
  (bind (_returnvalue_roll_3 _returnvalue_pitch_3) (`KismetMathLibrary.BreakRotator` (`Controller.GetControlRotation` _returnvalue)))
  (bind _yaw (.yaw (`KismetMathLibrary.Conv_VectorToRotator` Direction)))
  (`self.K2_SetActorRotation` (`KismetMathLibrary.RInterpTo_Constant` (`self.K2_GetActorRotation`) (`KismetMathLibrary.MakeRotator` 0.0 0.0 _yaw) DeltaTime InterpSpeed))
  (`Controller.SetControlRotation` _returnvalue (`KismetMathLibrary.MakeRotator` _returnvalue_roll_3 _returnvalue_pitch_3 _returnvalue_yaw))
  (return (`KismetMathLibrary.InRange_FloatFloat` _returnvalue_yaw_2 (- _yaw RotatedThreshold) (+ _yaw RotatedThreshold))))

(fn `ToggleInteractAttampt`
  (params (Enable :type Boolean))
  (returns (ReturnValue :type Boolean))
  (return false))

(fn `UserConstructionScript`
  (`parent.UserConstructionScript`))