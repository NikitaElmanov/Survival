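; BP_PainCausingZona is a zone actor that deals periodic damage to the player pawn while it is inside its box.
; Box overlap stores any entering actor as DamagedActor and, for the player pawn, starts a looping timer at PeriodDamage intervals.
; Each tick of that timer applies BaseDamage to the player, with the player's own controller as instigator.
; When the stored actor leaves, the timer and reference are cleared.
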(event `self.Box.OnComponentBeginOverlap`
  (params (OverlappedComponent :type "PrimitiveComponent Object Reference") (OtherActor :type "Actor Object Reference") (OtherComp :type "PrimitiveComponent Object Reference") (OtherBodyIndex :type Integer) (bFromSweep :type Boolean) (SweepResult :type "HitResult Structure (by ref)"))
  (bind _output_get (set `self.DamagedActor` OtherActor))
  (if (== _output_get (`GameplayStatics.GetPlayerPawn` 0))
    (bind _returnvalue (`KismetSystemLibrary.K2_SetTimer` null "ApplyDamageForCharacter" (`self.PeriodDamage`) true))
    (set `self.DamageCausingTimer` _returnvalue)))

(event `self.Box.OnComponentEndOverlap`
  (params (OverlappedComponent :type "PrimitiveComponent Object Reference") (OtherActor :type "Actor Object Reference") (OtherComp :type "PrimitiveComponent Object Reference") (OtherBodyIndex :type Integer))
  (if (== OtherActor (`self.DamagedActor`))
    (`KismetSystemLibrary.K2_ClearAndInvalidateTimerHandle` (`self.DamageCausingTimer`))
    (set `self.DamagedActor` null)))

(fn `ApplyDamageForCharacter`
  (`GameplayStatics.ApplyDamage` (`GameplayStatics.GetPlayerPawn` 0) (`self.BaseDamage`) (`GameplayStatics.GetPlayerController` 0) self))

(fn `UserConstructionScript`)