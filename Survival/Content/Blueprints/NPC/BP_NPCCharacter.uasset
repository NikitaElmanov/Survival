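; NPC character that can be alarmed, attack with its equipped weapon and expose its storage once dead.
; Player-caused damage triggers a one-time alarm that switches it to sprint speed and fires NPCAlarmed with the instigator.
; A helper yaws actor and controller toward a direction at constant speed, reporting arrival within a threshold.
; Interact on a corpse opens storage exchange only if the NPC's own controller casts to SurvivalPlayerController.
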(event `self.ReceiveAnyDamage`
  (params (Damage :type "Float (single-precision)") (DamageType :type "DamageType Object Reference") (InstigatedBy :type "Controller Object Reference") (DamageCauser :type "Actor Object Reference"))
  ;[1 1 1] Alarm by damage
  (`parent.ReceiveAnyDamage` Damage DamageType InstigatedBy DamageCauser)
  (if (== InstigatedBy (`GameplayStatics.GetPlayerController` 0))
    (`self.Alarm` (`GameplayStatics.GetPlayerCharacter` 0))))

(event `Attack`
  (params (Target :type "Actor Object Reference"))
  (`/Game/Blueprints/Storage/Items/Equipables/Weapons/Weapon.UseWeapon` (`/Game/Blueprints/Characters/BP_EquipComponent.Weapon` (`self.BP_EquipedComponent`)) true))

(event `StopAttack`
  (`/Game/Blueprints/Storage/Items/Equipables/Weapons/Weapon.UseWeapon` (`/Game/Blueprints/Characters/BP_EquipComponent.Weapon` (`self.BP_EquipedComponent`)) false))

(fn `Alarm`
  (params (Instigator :type "Pawn Object Reference"))
  (locals (L_Instiator :type "Pawn Object Reference"))
  (if (and (not (`self.Alarmed`)) (not (`self.Dead`)))
    (set `local.L_Instiator` Instigator)
    (set `self.Alarmed` true)
    (set `CharacterMovementComponent.MaxWalkSpeed` (`self.SprintingSpeed`) (`self.CharacterMovement`))
    (set `self.IsSprinting` true)
    (`self.NPCAlarmed` (`local.L_Instiator`))))

(fn `Interact`
  (params (Character :type "/Game/Blueprints/Characters/SurvivalCharacter Object Reference"))
  (returns (Successfull :type Boolean) (Message :type String))
  (if (`self.Dead`)
    (bind _assurvival_player_controller (cast `/Game/Blueprints/GameMode/SurvivalPlayerController` (`self.GetController`)))
    (`/Game/Blueprints/GameMode/SurvivalPlayerController.ExchangeWidget` _assurvival_player_controller (`self.BP_StorageComponent`) false)
    (return true "")
    (else
      (return false ""))))

(fn `RotateTowardsDirection`
  (params (DeltaTime :type "Float (double-precision)") (InterpSpeed :type "Float (double-precision)") (Direction :type "Vector Structure") (RotatedThreshold :type "Float (double-precision)"))
  (returns (Rotated :type Boolean))
  (bind (_returnvalue_roll _returnvalue_pitch _returnvalue_yaw) (`KismetMathLibrary.BreakRotator` (`self.K2_GetActorRotation`)))
  (bind _returnvalue (`self.GetController`))
  (bind (_returnvalue_roll_2 _returnvalue_pitch_2 _returnvalue_yaw_2) (`KismetMathLibrary.BreakRotator` (`self.K2_GetActorRotation`)))
  (bind (_returnvalue_roll_3 _returnvalue_pitch_3) (`KismetMathLibrary.BreakRotator` (`Controller.GetControlRotation` _returnvalue)))
  (bind _yaw (.yaw (`KismetMathLibrary.Conv_VectorToRotator` Direction)))
  (`self.K2_SetActorRotation` (`KismetMathLibrary.RInterpTo_Constant` (`self.K2_GetActorRotation`) (`KismetMathLibrary.MakeRotator` 0.0 0.0 _yaw) DeltaTime InterpSpeed))
  (`Controller.SetControlRotation` _returnvalue (`KismetMathLibrary.MakeRotator` _returnvalue_roll_3 _returnvalue_pitch_3 _returnvalue_yaw))
  (return (`KismetMathLibrary.InRange_FloatFloat` _returnvalue_yaw_2 (- _yaw RotatedThreshold) (+ _yaw RotatedThreshold))))

(fn `UserConstructionScript`
  (`parent.UserConstructionScript`))