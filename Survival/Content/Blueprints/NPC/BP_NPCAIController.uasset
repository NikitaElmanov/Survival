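; BP_NPCAIController is the AI controller for BP_NPCCharacter pawns.
; On possess it caches the NPC, initializes its follow component and binds to the NPC's alarmed and death events and the component's destination-reached event.
; The alarm handler only prints a debug message, and the death and destination-reached handlers are empty stubs.
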(event `self.ReceivePossess`
  (params (PossessedPawn :type "Pawn Object Reference"))
  (`self.Init`))

(fn `BindEvents`
  (add `/Game/Blueprints/NPC/BP_NPCCharacter.NPCAlarmed` (`self.NPC`) (`|CreateDelegate` :!event `NPCAlarm`))
  (add `/Game/Blueprints/Characters/SurvivalCharacter.CharDead` (`self.NPC`) (`|CreateDelegate` :!event `Dead`))
  (add `/Game/Blueprints/NPC/Components/NPCFollowComponent.DestReached` (`self.NPCFollowComponent`) (`|CreateDelegate` :!event `FollowDestReached`)))

(fn `Dead`)

(fn `FollowDestReached`)

(fn `Init`
  (bind _asbp_npccharacter (cast `/Game/Blueprints/NPC/BP_NPCCharacter` (`self.K2_GetPawn`)))
  (set `self.NPC` _asbp_npccharacter)
  (`/Game/Blueprints/NPC/Components/MainNPCControlComponent.Init` (`self.NPCFollowComponent`))
  (`self.BindEvents`))

(fn `NPCAlarm`
  (params (Instigator :type "Pawn Object Reference"))
  (`KismetSystemLibrary.PrintString` "NPC alarmed"))

(fn `UserConstructionScript`)