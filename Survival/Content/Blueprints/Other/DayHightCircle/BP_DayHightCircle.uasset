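; Day-night cycle actor that drives a level's sun, sky light, fog and sky sphere from a looping 24-hour Time value.
; Each tick advances Time by TimeSpeed, refreshes the sky sphere, rotates the directional light and arrow through a full turn, and prints Time on screen.
; Color curves sampled at Time tint the directional light, sky light and fog inscattering.
; The construction script runs the same update chain, applying the lighting at construction.
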(event `self.ReceiveTick`
  (params (DeltaSeconds :type "Float (single-precision)"))
  (`self.TimeCounter`)
  (`/Engine/EngineSky/BP_Sky_Sphere.UpdateSunDirection` (`self.SkySphere`))
  (`self.RotateDirLight`)
  (`self.SetDirLightColor`)
  (`self.SetDirSkyLightColor`)
  (`self.UpdateFogColor`)
  (`KismetSystemLibrary.PrintString` (`KismetStringLibrary.Conv_DoubleToString` (`self.Time`)) true true (struct :`G` 0.66 :`B` 1.0 :`A` 1.0) 0.0))

(fn `RotateDirLight`
  (bind _returnvalue (`KismetMathLibrary.MakeRotator` 0.0 (`KismetMathLibrary.Lerp` 90.0 450.0 (/ (`self.Time`) 24.0))))
  (`self.K2_SetActorRotation` (`self.DirLight`) _returnvalue false)
  (`SceneComponent.K2_SetWorldRotation` (`self.Arrow`) _returnvalue false false))

(fn `SetDirLightColor`
  (`LightComponent.SetLightColor` (`Light.LightComponent` (`self.DirLight`)) (`CurveLinearColor.GetLinearColorValue` (`self.LightColorCurve`) (`self.Time`)) false))

(fn `SetDirSkyLightColor`
  (`SkyLightComponent.SetLightColor` (`SkyLight.LightComponent` (`self.SkyLight`)) (`CurveLinearColor.GetLinearColorValue` (`self.SkyLightColorCurve`) (`self.Time`))))

(fn `TimeCounter`
  (bind _output_get (set `self.Time` (+ (`self.Time`) (* (`GameplayStatics.GetWorldDeltaSeconds`) (`self.TimeSpeed`)))))
  (if (>= _output_get 24.0)
    (set `self.Time` 0.0)))

(fn `UpdateFogColor`
  (`ExponentialHeightFogComponent.SetFogInscatteringColor` (`ExponentialHeightFog.Component` (`self.ExponentFog`)) (`CurveLinearColor.GetLinearColorValue` (`self.FogColorCurve`) (`self.Time`))))

(fn `UserConstructionScript`
  (`self.TimeCounter`)
  (`/Engine/EngineSky/BP_Sky_Sphere.UpdateSunDirection` (`self.SkySphere`))
  (`self.RotateDirLight`)
  (`self.SetDirLightColor`)
  (`self.SetDirSkyLightColor`)
  (`self.UpdateFogColor`))